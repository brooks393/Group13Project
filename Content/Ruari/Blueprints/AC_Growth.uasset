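; AC_Growth lets the player toggle a growth effect with the R key.
; A FlipFlop alternates between calling PlayGrowth on the Growth reference, printing a failure message if it is invalid, and attempting to shrink back.
; The shrink step line-traces upward from the player character on the Visibility channel with debug drawing, and calls ShrinkageToNormal only when the trace hits something.
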(event Input|KeyboardEvents|R
  (params (Key :type Key%20Structure :default "None"))
  (bind _returnvalue (Game|GetPlayerCharacter 0))
  (bind _growth (Variables|Default|Getgrowth))
  (bind _returnvalue_2 (Transformation|GetActorLocation _returnvalue))
  (:Pressed
    (Utilities|FlowControl|FlipFlop
      (:A
        (Utilities|IsValid _growth
          (:Is%20Valid
            (Default|PlayGrowth _growth))
          (:Is%20Not%20Valid
            (Development|PrintString "Growth Fail"))))
      (:B
        (bind _returnvalue_3 (Collision|LineTraceByChannel _returnvalue_2 (+ _returnvalue_2 (* (Transformation|GetActorUpVector (Game|GetPlayerCharacter 0)) 4e+02)) "TraceTypeQuery1" false (Utilities|Array|MakeArray (Game|GetPlayerCharacter 0)) "ForDuration"))
        (if _returnvalue_3
          (Default|ShrinkagetoNormal (Variables|Default|Getgrowth)))))))