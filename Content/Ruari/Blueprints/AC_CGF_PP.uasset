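; Work-in-progress logic for a fox, chicken and grain puzzle, tracking which items are in two areas.
; Pressing F sets the Glass material on the sphere of any Grain actor overlapping the player.
; Two mirrored custom events add to per-area arrays, then check combinations to print a win or failure.
; The array inputs are unconnected and the AreaA and AreaB functions are empty stubs.
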(event Custom|Area
  (bind _areab (Variables|Default|GetAreaB))
  (bind _areab_2 (Variables|Default|GetAreaB))
  (bind _returnvalue (Utilities|Array|ContainsItem _areab_2 0))
  (bind _returnvalue_2 (Utilities|Array|ContainsItem _areab_2 0))
  (bind _returnvalue_3 (Utilities|Array|ContainsItem _areab_2 0))
  (bind _returnvalue_4 (Utilities|Array|ContainsItem _areab_2 0))
  (bind _returnvalue_5 (and _returnvalue _returnvalue_2))
  (bind _returnvalue_6 (and _returnvalue_4 _returnvalue_3))
  (Utilities|Array|Add _areab 0)
  (for _array_element _areab
    (if (and _returnvalue_5 _returnvalue_6)
      (Development|PrintString "U Win")
      (elif _returnvalue_6
        (Development|PrintText "failure")
        (elif _returnvalue_5
          (Development|PrintText "failure"))))))

(event Custom|CustomEvent
  (bind _area_a (Variables|Default|GetArea%20A))
  (bind _area_a_2 (Variables|Default|GetArea%20A))
  (bind _returnvalue (Utilities|Array|ContainsItem _area_a_2 0))
  (bind _returnvalue_2 (Utilities|Array|ContainsItem _area_a_2 0))
  (bind _returnvalue_3 (Utilities|Array|ContainsItem _area_a_2 0))
  (bind _returnvalue_4 (Utilities|Array|ContainsItem _area_a_2 0))
  (bind _returnvalue_5 (and _returnvalue_4 _returnvalue_3))
  (bind _returnvalue_6 (and _returnvalue _returnvalue_2))
  ;[0.15 0.15 0.15 0.5] On Begin Event Overlap + get actor (which overlaps add into array)
  (Utilities|Array|Add _area_a 0)
  (for _array_element _area_a
    (if (and _returnvalue_6 _returnvalue_5)
      (Development|PrintString "U Win")
      (elif _returnvalue_5
        (Development|PrintText "failure")
        (elif _returnvalue_6
          (Development|PrintText "failure"))))))

(event Input|KeyboardEvents|F
  (params (Key :type Key%20Structure :default "None"))
  (:Pressed
    (for _array_element (Collision|GetOverlappingActors (Game|GetPlayerCharacter 0) "/Game/Ruari/Blueprints/CGF_Puzzle_Proto/Grain.Grain_C" :!class /Script/Engine.Actor)
      (Rendering|Material|SetMaterial (Variables|/Game/Ruari/Blueprints/CGF_Puzzle_Proto/Grain.Grain_C|GetSphere _array_element) 0 "/Game/Brandon/Bookcase/Glass.Glass"))))

(fn AreaA)

(fn AreaB)