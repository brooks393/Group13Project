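; Fox, chicken and grain river-crossing puzzle prototype, viewed through its own camera when used.
; Tick traces under the cursor; hovering an item teleports it between sides via FlipFlop, gated by a LastInteractionTime check.
; Per-side mesh arrays are checked after moves: all three together wins, chicken with grain or fox alone loses.
; Either result restores LevelCamera and sets a good or bad Background material; older movement experiments remain unwired.
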(event OnComponentBeginOverlap(AreaB)
  (params (OverlappedComponent :type Primitive%20Component%20Object%20Reference) (OtherActor :type Actor%20Object%20Reference) (OtherComp :type Primitive%20Component%20Object%20Reference) (OtherBodyIndex :type Integer) (bFromSweep :type Boolean) (SweepResult :type Hit%20Result%20Structure%20%28by%20ref%29))
  ;[1 0 0] GRAVEYARD *NOT IN USE
  ;;[0.15 0.15 0.15 0.5] Logic for win/loose
  ;;;[0.15 0.15 0.15 0.5] checks other area if has certain items within the area
)

(event OnComponentBeginOverlap(I_A_Grain)
  (params (OverlappedComponent :type Primitive%20Component%20Object%20Reference) (OtherActor :type Actor%20Object%20Reference) (OtherComp :type Primitive%20Component%20Object%20Reference) (OtherBodyIndex :type Integer) (bFromSweep :type Boolean) (SweepResult :type Hit%20Result%20Structure%20%28by%20ref%29))
  ;[0.838 0.07726 1 0.5] Using
  ;;[0.15 0.15 0.15 0.5] Moving the Components
  ;;;[0.15 0.15 0.15 0.5] Grain moving to opposite side
)

(event OnComponentBeginOverlap(AreaA)
  (params (OverlappedComponent :type Primitive%20Component%20Object%20Reference) (OtherActor :type Actor%20Object%20Reference) (OtherComp :type Primitive%20Component%20Object%20Reference) (OtherBodyIndex :type Integer) (bFromSweep :type Boolean) (SweepResult :type Hit%20Result%20Structure%20%28by%20ref%29))
  (bind _area_a (Variables|Default|GetArea%20A))
  (bind _area_a_2 (Variables|Default|GetArea%20A))
  (bind _chicken (Variables|Components|GetChicken))
  (bind _grain (Variables|Components|GetGrain))
  (bind _fox (Variables|Components|GetFox))
  (bind _staticmesh (Variables|/Script/Engine.StaticMeshComponent|GetStaticMesh _chicken))
  (bind _staticmesh_2 (Variables|/Script/Engine.StaticMeshComponent|GetStaticMesh _grain))
  (bind _staticmesh_3 (Variables|/Script/Engine.StaticMeshComponent|GetStaticMesh _fox))
  (bind _returnvalue (Utilities|Array|ContainsItem _area_a_2 _staticmesh_2))
  (bind _returnvalue_2 (Utilities|Array|ContainsItem _area_a_2 _staticmesh))
  (bind _returnvalue_3 (Utilities|Array|ContainsItem _area_a_2 _staticmesh))
  (bind _returnvalue_4 (Utilities|Array|ContainsItem _area_a_2 _staticmesh_3))
  (bind _returnvalue_5 (and _returnvalue_3 _returnvalue_4))
  (bind _returnvalue_6 (and _returnvalue _returnvalue_2))
  ;[1 0 0] GRAVEYARD *NOT IN USE
  ;;[0.15 0.15 0.15 0.5] Logic for win/loose
  ;;;[0.15 0.15 0.15 0.5] checks if one area has certain items within an area
  ;;;;[0.15 0.15 0.15 0.5] On Begin Event Overlap + get actor (which overlaps add into array)
  (Utilities|Array|Add _area_a 0)
  (for _array_element _area_a
    (if (and _returnvalue_5 _returnvalue_6)
      (Development|PrintString "U Win")
      (elif _returnvalue_6
        (Development|PrintText "failure")
        (elif _returnvalue_5
          (Development|PrintText "failure"))))))

(event Custom|CustomEvent_1
  (params (OverlappedComponent :type Primitive%20Component%20Object%20Reference) (OtherActor :type Actor%20Object%20Reference) (OtherComp :type Primitive%20Component%20Object%20Reference) (OtherBodyIndex :type Integer) (bFromSweep :type Boolean) (SweepResult :type Hit%20Result%20Structure%20%28by%20ref%29))
  ;[1 0 0] GRAVEYARD *NOT IN USE
  ;;[0.15 0.15 0.15 0.5] WIP2 - item movement v2
)

(event Custom|LeaveGAem
  (bind _chicken (Variables|Components|GetChicken))
  (bind _area_a (Variables|Default|GetArea%20A))
  (bind _chicken_2 (Variables|Components|GetChicken))
  (bind _areab_0 (Variables|Default|GetAreaB_0))
  (bind _staticmesh (Variables|/Script/Engine.StaticMeshComponent|GetStaticMesh _chicken_2))
  (bind _staticmesh_2 (Variables|/Script/Engine.StaticMeshComponent|GetStaticMesh _chicken))
  ;[0.838 0.07726 1 0.5] Using
  ;;[0.15 0.15 0.15 0.5] setting camera view
  (for _array_element (Variables|Default|GetWin)
    _)
  (if true
    (Game|Player|SetViewTargetwithBlend (Game|GetPlayerController 0) (Variables|Default|GetLevelCamera) 0.0 "VTBlend_Linear" 0.0 false)
    (if (or (and (and (Utilities|Array|ContainsItem _area_a _staticmesh) (Utilities|Array|ContainsItem _area_a (Variables|/Script/Engine.StaticMeshComponent|GetStaticMesh (Variables|Components|GetFox)))) (and (Utilities|Array|ContainsItem _area_a (Variables|/Script/Engine.StaticMeshComponent|GetStaticMesh (Variables|Components|GetGrain))) (Utilities|Array|ContainsItem _area_a _staticmesh))) (and (and (Utilities|Array|ContainsItem _areab_0 _staticmesh_2) (Utilities|Array|ContainsItem _areab_0 (Variables|/Script/Engine.StaticMeshComponent|GetStaticMesh (Variables|Components|GetFox)))) (and (Utilities|Array|ContainsItem _areab_0 (Variables|/Script/Engine.StaticMeshComponent|GetStaticMesh (Variables|Components|GetGrain))) (Utilities|Array|ContainsItem _areab_0 _staticmesh_2))))
      ;;;[0.15 0.15 0.15 0.5] Good
      (Rendering|Material|SetMaterial (Variables|Default|Getbackground) 0 "/Game/Rey/StaticMeshes/pasted__Hour2.pasted__Hour2")
      (else
        ;;;[0.15 0.15 0.15 0.5] Bad
        (Rendering|Material|SetMaterial (Variables|Default|Getbackground) 0 "/Game/Rey/StaticMeshes/pasted__faceBasebottom2.pasted__faceBasebottom2")))))

(event Custom|Move%20Chicken
  (params (OtherActor :type Actor%20Object%20Reference))
  (bind _chicken (Variables|Components|GetChicken))
  (bind _chicken_2 (Variables|Components|GetChicken))
  (bind _chicken_3 (Variables|Components|GetChicken))
  (bind _fox (Variables|Components|GetFox))
  (bind _area_a (Variables|Default|GetArea%20A))
  (bind _chicken_4 (Variables|Components|GetChicken))
  (bind _grain (Variables|Components|GetGrain))
  (bind _fox_2 (Variables|Components|GetFox))
  (bind _grain_2 (Variables|Components|GetGrain))
  (bind _areab_0 (Variables|Default|GetAreaB_0))
  (bind _returnvalue (Transformation|GetWorldLocation _chicken_2))
  (bind _returnvalue_2 (Transformation|GetWorldLocation _chicken))
  (bind _staticmesh (Variables|/Script/Engine.StaticMeshComponent|GetStaticMesh _fox))
  (bind _staticmesh_2 (Variables|/Script/Engine.StaticMeshComponent|GetStaticMesh _chicken_4))
  (bind _staticmesh_3 (Variables|/Script/Engine.StaticMeshComponent|GetStaticMesh _grain))
  (bind _staticmesh_4 (Variables|/Script/Engine.StaticMeshComponent|GetStaticMesh _fox_2))
  (bind _staticmesh_5 (Variables|/Script/Engine.StaticMeshComponent|GetStaticMesh _chicken_3))
  (bind _staticmesh_6 (Variables|/Script/Engine.StaticMeshComponent|GetStaticMesh _chicken_2))
  (bind _staticmesh_7 (Variables|/Script/Engine.StaticMeshComponent|GetStaticMesh _grain_2))
  (bind _returnvalue_3 (Utilities|Array|ContainsItem _area_a _staticmesh_2))
  (bind _returnvalue_4 (Utilities|Array|ContainsItem _area_a _staticmesh_2))
  (bind _returnvalue_5 (Utilities|Array|ContainsItem _area_a _staticmesh_4))
  (bind _returnvalue_6 (Utilities|Array|ContainsItem _area_a _staticmesh_3))
  (bind _returnvalue_7 (Utilities|Array|ContainsItem _areab_0 _staticmesh_7))
  (bind _returnvalue_8 (Utilities|Array|ContainsItem _areab_0 _staticmesh_5))
  (bind _returnvalue_9 (Utilities|Array|ContainsItem _areab_0 _staticmesh_5))
  (bind _returnvalue_10 (Utilities|Array|ContainsItem _areab_0 _staticmesh))
  (bind _returnvalue_11 (and _returnvalue_4 _returnvalue_5))
  (bind _returnvalue_12 (and _returnvalue_7 _returnvalue_8))
  (bind _returnvalue_13 (and _returnvalue_6 _returnvalue_3))
  (bind _returnvalue_14 (and _returnvalue_9 _returnvalue_10))
  ;[0.838 0.07726 1 0.5] Using
  ;;[0.15 0.15 0.15 0.5] Moving the Components
  ;;;[0.15 0.15 0.15 0.5] Moving the Chicken
  (if (>= (- (Utilities|Time|GetGameTimeinSeconds) (Variables|Default|GetLastInteractionTime)) 2.0)
    (Utilities|Array|RemoveItem (Variables|Default|GetArea%20A) _staticmesh_6)
    (Utilities|Array|RemoveItem (Variables|Default|GetAreaB_0) _staticmesh_6)
    (Utilities|FlowControl|FlipFlop
      (:A
        (Transformation|SetWorldLocation _chicken_2 (Math|Vector|MakeVector (+ (.x _returnvalue) 3.2e+02) (.y _returnvalue) (.z _returnvalue)) false true)
        (Utilities|Array|Add (Variables|Default|GetAreaB_0) (Variables|/Script/Engine.StaticMeshComponent|GetStaticMesh _chicken_2))
        ;;[0.15 0.15 0.15 0.5] lOGIC
        ;;;[0.15 0.15 0.15 0.5] checks other area if has certain items within the area
        (for _array_element (Variables|Default|GetAreaB_0)
          (if (and _returnvalue_14 _returnvalue_12)
            (Variables|Default|SetWin (Variables|Default|GetWin))
            (Development|PrintString "U Win")
            (CallFunction|LeaveGAem)
            (elif _returnvalue_12
              (Variables|Default|SetLoss (Variables|Default|GetLoss))
              (Development|PrintText "failure")
              (CallFunction|LeaveGAem)
              (elif _returnvalue_14
                (Variables|Default|SetLoss (Variables|Default|GetLoss))
                (Development|PrintText "failure")
                (CallFunction|LeaveGAem))))))
      (:B
        (Transformation|SetWorldLocation _chicken (Math|Vector|MakeVector (+ (.x _returnvalue_2) -3.2e+02) (.y _returnvalue_2) (.z _returnvalue_2)) false true)
        (Utilities|Array|Add (Variables|Default|GetArea%20A) (Variables|/Script/Engine.StaticMeshComponent|GetStaticMesh _chicken))
        ;;;[0.15 0.15 0.15 0.5] checks if one area has certain items within an area
        (for _array_element_2 (Variables|Default|GetArea%20A)
          (if (and _returnvalue_11 _returnvalue_13)
            (Variables|Default|SetWin (Variables|Default|GetWin))
            ;;;;[0.15 0.15 0.15 0.5] One loose condition
            (Development|PrintString "U Win")
            (CallFunction|LeaveGAem)
            (elif _returnvalue_13
              (Variables|Default|SetLoss (Variables|Default|GetLoss))
              (Development|PrintText "failure")
              (CallFunction|LeaveGAem)
              (elif _returnvalue_11
                (Variables|Default|SetLoss (Variables|Default|GetLoss))
                (Development|PrintText "failure")
                (CallFunction|LeaveGAem)))))))))

(event Custom|MoveGrain
  (params (OtherActor :type Actor%20Object%20Reference))
  (bind _chicken (Variables|Components|GetChicken))
  (bind _fox (Variables|Components|GetFox))
  (bind _area_a (Variables|Default|GetArea%20A))
  (bind _chicken_2 (Variables|Components|GetChicken))
  (bind _grain (Variables|Components|GetGrain))
  (bind _fox_2 (Variables|Components|GetFox))
  (bind _grain_2 (Variables|Components|GetGrain))
  (bind _areab_0 (Variables|Default|GetAreaB_0))
  (bind _grain_3 (Variables|Components|GetGrain))
  (bind _grain_4 (Variables|Components|GetGrain))
  (bind _returnvalue (Transformation|GetWorldLocation _grain_3))
  (bind _returnvalue_2 (Transformation|GetWorldLocation _grain_4))
  (bind _staticmesh (Variables|/Script/Engine.StaticMeshComponent|GetStaticMesh _fox))
  (bind _staticmesh_2 (Variables|/Script/Engine.StaticMeshComponent|GetStaticMesh _chicken_2))
  (bind _staticmesh_3 (Variables|/Script/Engine.StaticMeshComponent|GetStaticMesh _grain))
  (bind _staticmesh_4 (Variables|/Script/Engine.StaticMeshComponent|GetStaticMesh _fox_2))
  (bind _staticmesh_5 (Variables|/Script/Engine.StaticMeshComponent|GetStaticMesh _chicken))
  (bind _staticmesh_6 (Variables|/Script/Engine.StaticMeshComponent|GetStaticMesh _grain_2))
  (bind _staticmesh_7 (Variables|/Script/Engine.StaticMeshComponent|GetStaticMesh _grain_3))
  (bind _returnvalue_3 (Utilities|Array|ContainsItem _area_a _staticmesh_2))
  (bind _returnvalue_4 (Utilities|Array|ContainsItem _area_a _staticmesh_2))
  (bind _returnvalue_5 (Utilities|Array|ContainsItem _area_a _staticmesh_4))
  (bind _returnvalue_6 (Utilities|Array|ContainsItem _area_a _staticmesh_3))
  (bind _returnvalue_7 (Utilities|Array|ContainsItem _areab_0 _staticmesh_6))
  (bind _returnvalue_8 (Utilities|Array|ContainsItem _areab_0 _staticmesh_5))
  (bind _returnvalue_9 (Utilities|Array|ContainsItem _areab_0 _staticmesh_5))
  (bind _returnvalue_10 (Utilities|Array|ContainsItem _areab_0 _staticmesh))
  (bind _returnvalue_11 (and _returnvalue_4 _returnvalue_5))
  (bind _returnvalue_12 (and _returnvalue_7 _returnvalue_8))
  (bind _returnvalue_13 (and _returnvalue_6 _returnvalue_3))
  (bind _returnvalue_14 (and _returnvalue_9 _returnvalue_10))
  ;[0.838 0.07726 1 0.5] Using
  ;;[0.15 0.15 0.15 0.5] Moving the Components
  ;;;[0.15 0.15 0.15 0.5] Grain moving to opposite side
  (if (>= (- (Utilities|Time|GetGameTimeinSeconds) (Variables|Default|GetLastInteractionTime)) 2.0)
    (Utilities|Array|RemoveItem (Variables|Default|GetArea%20A) _staticmesh_7)
    (Utilities|Array|RemoveItem (Variables|Default|GetAreaB_0) _staticmesh_7)
    (Utilities|FlowControl|FlipFlop
      (:A
        (Transformation|SetWorldLocation _grain_3 (Math|Vector|MakeVector (+ (.x _returnvalue) 3.2e+02) (.y _returnvalue) (.z _returnvalue)) false true)
        (Utilities|Array|Add (Variables|Default|GetAreaB_0) (Variables|/Script/Engine.StaticMeshComponent|GetStaticMesh _grain_3))
        ;;[0.15 0.15 0.15 0.5] lOGIC
        ;;;[0.15 0.15 0.15 0.5] checks other area if has certain items within the area
        (for _array_element (Variables|Default|GetAreaB_0)
          (if (and _returnvalue_14 _returnvalue_12)
            (Variables|Default|SetWin (Variables|Default|GetWin))
            (Development|PrintString "U Win")
            (CallFunction|LeaveGAem)
            (elif _returnvalue_12
              (Variables|Default|SetLoss (Variables|Default|GetLoss))
              (Development|PrintText "failure")
              (CallFunction|LeaveGAem)
              (elif _returnvalue_14
                (Variables|Default|SetLoss (Variables|Default|GetLoss))
                (Development|PrintText "failure")
                (CallFunction|LeaveGAem))))))
      (:B
        (Transformation|SetWorldLocation _grain_4 (Math|Vector|MakeVector (+ (.x _returnvalue_2) -3.2e+02) (.y _returnvalue_2) (.z _returnvalue_2)) false true)
        (Utilities|Array|Add (Variables|Default|GetArea%20A) (Variables|/Script/Engine.StaticMeshComponent|GetStaticMesh _grain_4))
        ;;;[0.15 0.15 0.15 0.5] checks if one area has certain items within an area
        (for _array_element_2 (Variables|Default|GetArea%20A)
          (if (and _returnvalue_11 _returnvalue_13)
            (Variables|Default|SetWin (Variables|Default|GetWin))
            ;;;;[0.15 0.15 0.15 0.5] One loose condition
            (Development|PrintString "U Win")
            (CallFunction|LeaveGAem)
            (elif _returnvalue_13
              (Variables|Default|SetLoss (Variables|Default|GetLoss))
              (Development|PrintText "failure")
              (CallFunction|LeaveGAem)
              (elif _returnvalue_11
                (Variables|Default|SetLoss (Variables|Default|GetLoss))
                (Development|PrintText "failure")
                (CallFunction|LeaveGAem)))))))))

(event Custom|Move%20Fox
  (params (OtherActor :type Actor%20Object%20Reference))
  (bind _chicken (Variables|Components|GetChicken))
  (bind _fox (Variables|Components|GetFox))
  (bind _area_a (Variables|Default|GetArea%20A))
  (bind _chicken_2 (Variables|Components|GetChicken))
  (bind _grain (Variables|Components|GetGrain))
  (bind _fox_2 (Variables|Components|GetFox))
  (bind _grain_2 (Variables|Components|GetGrain))
  (bind _areab_0 (Variables|Default|GetAreaB_0))
  (bind _fox_3 (Variables|Components|GetFox))
  (bind _fox_4 (Variables|Components|GetFox))
  (bind _returnvalue (Transformation|GetWorldLocation _fox_3))
  (bind _returnvalue_2 (Transformation|GetWorldLocation _fox_4))
  (bind _staticmesh (Variables|/Script/Engine.StaticMeshComponent|GetStaticMesh _fox_3))
  (bind _staticmesh_2 (Variables|/Script/Engine.StaticMeshComponent|GetStaticMesh _fox))
  (bind _staticmesh_3 (Variables|/Script/Engine.StaticMeshComponent|GetStaticMesh _chicken_2))
  (bind _staticmesh_4 (Variables|/Script/Engine.StaticMeshComponent|GetStaticMesh _grain))
  (bind _staticmesh_5 (Variables|/Script/Engine.StaticMeshComponent|GetStaticMesh _fox_2))
  (bind _staticmesh_6 (Variables|/Script/Engine.StaticMeshComponent|GetStaticMesh _chicken))
  (bind _staticmesh_7 (Variables|/Script/Engine.StaticMeshComponent|GetStaticMesh _grain_2))
  (bind _returnvalue_3 (Utilities|Array|ContainsItem _area_a _staticmesh_3))
  (bind _returnvalue_4 (Utilities|Array|ContainsItem _area_a _staticmesh_3))
  (bind _returnvalue_5 (Utilities|Array|ContainsItem _area_a _staticmesh_5))
  (bind _returnvalue_6 (Utilities|Array|ContainsItem _area_a _staticmesh_4))
  (bind _returnvalue_7 (Utilities|Array|ContainsItem _areab_0 _staticmesh_7))
  (bind _returnvalue_8 (Utilities|Array|ContainsItem _areab_0 _staticmesh_6))
  (bind _returnvalue_9 (Utilities|Array|ContainsItem _areab_0 _staticmesh_6))
  (bind _returnvalue_10 (Utilities|Array|ContainsItem _areab_0 _staticmesh_2))
  (bind _returnvalue_11 (and _returnvalue_4 _returnvalue_5))
  (bind _returnvalue_12 (and _returnvalue_7 _returnvalue_8))
  (bind _returnvalue_13 (and _returnvalue_6 _returnvalue_3))
  (bind _returnvalue_14 (and _returnvalue_9 _returnvalue_10))
  ;[0.838 0.07726 1 0.5] Using
  ;;[0.15 0.15 0.15 0.5] Moving the Components
  ;;;[0.15 0.15 0.15 0.5] Moving Fox to other side
  (if (>= (- (Utilities|Time|GetGameTimeinSeconds) (Variables|Default|GetLastInteractionTime)) 2.0)
    (Utilities|Array|RemoveItem (Variables|Default|GetArea%20A) _staticmesh)
    (Utilities|Array|RemoveItem (Variables|Default|GetAreaB_0) _staticmesh)
    (Utilities|FlowControl|FlipFlop
      (:A
        (Transformation|SetWorldLocation _fox_3 (Math|Vector|MakeVector (+ (.x _returnvalue) 3.2e+02) (.y _returnvalue) (.z _returnvalue)) false true)
        (Utilities|Array|Add (Variables|Default|GetAreaB_0) (Variables|/Script/Engine.StaticMeshComponent|GetStaticMesh _fox_3))
        ;;[0.15 0.15 0.15 0.5] lOGIC
        ;;;[0.15 0.15 0.15 0.5] checks other area if has certain items within the area
        (for _array_element (Variables|Default|GetAreaB_0)
          (if (and _returnvalue_14 _returnvalue_12)
            (Variables|Default|SetWin (Variables|Default|GetWin))
            (Development|PrintString "U Win")
            (CallFunction|LeaveGAem)
            (elif _returnvalue_12
              (Variables|Default|SetLoss (Variables|Default|GetLoss))
              (Development|PrintText "failure")
              (CallFunction|LeaveGAem)
              (elif _returnvalue_14
                (Variables|Default|SetLoss (Variables|Default|GetLoss))
                (Development|PrintText "failure")
                (CallFunction|LeaveGAem))))))
      (:B
        (Transformation|SetWorldLocation _fox_4 (Math|Vector|MakeVector (+ (.x _returnvalue_2) -3.2e+02) (.y _returnvalue_2) (.z _returnvalue_2)) false true)
        (Utilities|Array|Add (Variables|Default|GetArea%20A) (Variables|/Script/Engine.StaticMeshComponent|GetStaticMesh _fox_4))
        ;;;[0.15 0.15 0.15 0.5] checks if one area has certain items within an area
        (for _array_element_2 (Variables|Default|GetArea%20A)
          (if (and _returnvalue_11 _returnvalue_13)
            (Variables|Default|SetWin (Variables|Default|GetWin))
            ;;;;[0.15 0.15 0.15 0.5] One loose condition
            (Development|PrintString "U Win")
            (CallFunction|LeaveGAem)
            (elif _returnvalue_13
              (Variables|Default|SetLoss (Variables|Default|GetLoss))
              (Development|PrintText "failure")
              (CallFunction|LeaveGAem)
              (elif _returnvalue_11
                (Variables|Default|SetLoss (Variables|Default|GetLoss))
                (Development|PrintText "failure")
                (CallFunction|LeaveGAem)))))))))

(event EventTick
  (params (DeltaSeconds :type Float%20%28single-precision%29))
  (bind _returnvalue (Game|GetPlayerController 0))
  (bind _hitresult (Game|Player|GetHitResultUnderCursorbyChannel _returnvalue "TraceTypeQuery1" true))
  (bind (_bblockinghit _binitialoverlap _time _distance _location _impactpoint _normal _impactnormal _physmat _hitactor _hitcomponent) (Collision|BreakHitResult _hitresult))
  ;[0.838 0.07726 1 0.5] Using
  ;;[0.15 0.15 0.15 0.5] Brandon's mouse movement applied
  (Variables|/Script/Engine.PlayerController|SetbShowMouseCursor _returnvalue true)
  (if (== _hitcomponent (Variables|Components|GetGrain))
    (CallFunction|MoveGrain _hitactor)
    (elif (== _hitcomponent (Variables|Components|GetChicken))
      (CallFunction|MoveChicken _hitactor)
      (elif (== _hitcomponent (Variables|Components|GetFox))
        (CallFunction|MoveFox _hitactor)))))

(event EventBeginPlay
  ;[0.838 0.07726 1 0.5] Using
  ;;[0.15 0.15 0.15 0.5] Brandon's mouse movement applied
  (Input|SetInputModeGameandUI (Game|GetPlayerController 0) 0 "DoNotLock" true false))

(event EventItemUsed
  ;[0.838 0.07726 1 0.5] Using
  ;;[0.15 0.15 0.15 0.5] setting camera view
  (Game|Player|SetViewTargetwithBlend (Game|GetPlayerController 0) self 0.0 "VTBlend_Linear" 0.0 false))

(fn ConstructionScript)