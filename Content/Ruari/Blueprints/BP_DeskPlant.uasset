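; Desk plant Blueprint that animates growth through three plant models in a repeating cycle, starting on BeginPlay.
; Two timelines lerp the scale of the first and second models in turn, with delays before visibility toggles swap in the next model.
; After the third model's swap, the GrowthProgression flag loops execution back to reset the first two models' scales and restart the cycle.
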(event EventBeginPlay
  (if (Variables|Default|GetGrowth%20progression) :!label _label
    ;[0.15 0.15 0.15 0.5] Resets model's sizes
    (Transformation|SetRelativeScale3D (Variables|Default|Getplant) "1.000000,1.000000,1.000000")
    (Transformation|SetRelativeScale3D (Variables|Default|GetPlant%202%20) "1.000000,1.000000,1.000000")
    (Variables|Default|SetGrowth%20progression false)
    (goto _label)
    (else
      (Rendering|ToggleVisibility (Variables|Default|GetPlant%202%20) false)
      (Rendering|ToggleVisibility (Variables|Default|GetPlant%203) false)
      ;[0.15 0.15 0.15 0.5] Changes the actual scale of the plant
      (bind _growthspeed (Timeline|Timeline_8 PlayFromStart)
        (:Update
          (Transformation|SetRelativeScale3D (Variables|Default|Getplant) (Math|Vector|Lerp(Vector) (Variables|Default|GetPlantSizeNorm) (Variables|Default|GetPlantSizeProg) _growthspeed))
          (Utilities|FlowControl|Delay 6.0)
          ;[0.15 0.15 0.15 0.5] Deletes and Replaces with new model
          (Rendering|ToggleVisibility (Variables|Default|Getplant) false)
          (Rendering|ToggleVisibility (Variables|Default|GetPlant%202%20) false)
          ;[0.15 0.15 0.15 0.5] Changes the size of plant 2
          (Utilities|FlowControl|Delay 1.0)
          (bind _growthspeed_2 (Timeline|Timeline PlayFromStart)
            (:Update
              (Transformation|SetRelativeScale3D (Variables|Default|GetPlant%202%20) (Math|Vector|Lerp(Vector) (Variables|Default|GetPlantSizeNorm) (Variables|Default|GetPlantSizeProg) _growthspeed_2))
              (Utilities|FlowControl|Delay 3.0)
              ;[0.15 0.15 0.15 0.5] Destroys plant 2, replaces with plant 3
              (Rendering|ToggleVisibility (Variables|Default|GetPlant%202%20) false)
              (Rendering|ToggleVisibility (Variables|Default|GetPlant%203) false)
              (Variables|Default|SetGrowth%20progression true)
              (goto _label))))))))

(fn ConstructionScript)