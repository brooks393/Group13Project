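; Player shrink ability, named as an actor component, that toggles the player character between shrinking and growing back on the E key.
; BeginPlay caches the level's BP_ShrinkTimeline actor, which plays and reverses the shrink.
; Growing back requires a clear 200-unit upward visibility trace, drawn for debugging.
; The FlipFlop still advances when that trace is blocked, so the next press calls shrink again.
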(event EventBeginPlay
  (bind _returnvalue (Actor|GetActorOfClass "/Game/Ruari/Blueprints/BP_ShrinkTimeline.BP_ShrinkTimeline_C"))
  (Variables|Default|SetTimeline _returnvalue))

(event Input|KeyboardEvents|E
  (params (Key :type Key%20Structure :default "None"))
  (bind _returnvalue (Game|GetPlayerCharacter 0))
  (bind _timeline (Variables|Default|GetTimeline))
  (bind _returnvalue_2 (Transformation|GetActorLocation _returnvalue))
  ;[0.15 0.15 0.15 0.5] Shrinking
  (:Pressed
    (Utilities|FlowControl|FlipFlop
      (:A
        (Utilities|IsValid _timeline
          (:Is%20Valid
            (Default|PlayShrink _timeline (Game|GetPlayerCharacter 0)))
          (:Is%20Not%20Valid
            (Development|PrintString "Shrink Fail"))))
      (:B
        (bind _returnvalue_3 (Collision|LineTraceByChannel _returnvalue_2 (+ _returnvalue_2 (* (Transformation|GetActorUpVector (Game|GetPlayerCharacter 0)) 2e+02)) "TraceTypeQuery1" false (Utilities|Array|MakeArray (Game|GetPlayerCharacter 0)) "ForDuration"))
        (if (not _returnvalue_3)
          (Default|ReverseShrink (Variables|Default|GetTimeline) (Game|GetPlayerCharacter 0)))))))