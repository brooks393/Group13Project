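; One-way platform actor that lets Characters tagged "OneWay" jump up through it or drop down through it.
; Entering the lower trigger disables platform collision and launches the character, and the upper exit trigger restores collision.
; Overlapping the drop trigger enables input and opens a gate, so Left Ctrl disables platform and GoUp collision.
; A final drop trigger restores both.
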(event OnComponentBeginOverlap(Go_Up)
  (params (OverlappedComponent :type Primitive%20Component%20Object%20Reference) (OtherActor :type Actor%20Object%20Reference) (OtherComp :type Primitive%20Component%20Object%20Reference) (OtherBodyIndex :type Integer) (bFromSweep :type Boolean) (SweepResult :type Hit%20Result%20Structure%20%28by%20ref%29))
  ;[0.15 0.15 0.15 0.5] Jump up Through Platform
  (if (Actor|ActorHasTag OtherActor "OneWay")
    (Collision|SetCollisionEnabled (Variables|Default|GetPlatform) "NoCollision")
    (bind _ascharacter (Utilities|Casting|CastToCharacter OtherActor))
    (Character|LaunchCharacter _ascharacter (Variables|Default|GetLaunch%20Velocity) false false)))

(event OnComponentBeginOverlap(Go_Up_Final)
  (params (OverlappedComponent :type Primitive%20Component%20Object%20Reference) (OtherActor :type Actor%20Object%20Reference) (OtherComp :type Primitive%20Component%20Object%20Reference) (OtherBodyIndex :type Integer) (bFromSweep :type Boolean) (SweepResult :type Hit%20Result%20Structure%20%28by%20ref%29))
  ;[0.15 0.15 0.15 0.5] Jump up Through Platform
  (if (Actor|ActorHasTag OtherActor "OneWay")
    (Collision|SetCollisionEnabled (Variables|Default|GetPlatform) "QueryAndPhysics")))

(event OnComponentBeginOverlap(Go_down)
  (params (OverlappedComponent :type Primitive%20Component%20Object%20Reference) (OtherActor :type Actor%20Object%20Reference) (OtherComp :type Primitive%20Component%20Object%20Reference) (OtherBodyIndex :type Integer) (bFromSweep :type Boolean) (SweepResult :type Hit%20Result%20Structure%20%28by%20ref%29))
  ;[0.15 0.15 0.15 0.5] Go Down through platform
  (if (Actor|ActorHasTag OtherActor "OneWay")
    (Input|EnableInput self (Game|GetPlayerController 0))
    (Utilities|FlowControl|Gate true) ; enters at Open
  ))

(event OnComponentBeginOverlap(Go_Down_Final)
  (params (OverlappedComponent :type Primitive%20Component%20Object%20Reference) (OtherActor :type Actor%20Object%20Reference) (OtherComp :type Primitive%20Component%20Object%20Reference) (OtherBodyIndex :type Integer) (bFromSweep :type Boolean) (SweepResult :type Hit%20Result%20Structure%20%28by%20ref%29))
  ;[0.15 0.15 0.15 0.5] Go Down through platform
  (if (and (Actor|ActorHasTag OtherActor "OneWay") (not (Class|PrimitiveComponent|IsCollisionEnabled (Variables|Default|GetPlatform))))
    (Collision|SetCollisionEnabled (Variables|Default|GetPlatform) "QueryAndPhysics")))

(event OnComponentEndOverlap(Go_down)
  (params (OverlappedComponent :type Primitive%20Component%20Object%20Reference) (OtherActor :type Actor%20Object%20Reference) (OtherComp :type Primitive%20Component%20Object%20Reference) (OtherBodyIndex :type Integer))
  ;[0.15 0.15 0.15 0.5] Go Down through platform
  (if (Actor|ActorHasTag OtherActor "OneWay")
    (Input|DisableInput self (Game|GetPlayerController 0))
    (Utilities|FlowControl|Gate true) ; enters at Close
  ))

(event Input|KeyboardEvents|LeftCtrl
  (params (Key :type Key%20Structure :default "None"))
  ;[0.15 0.15 0.15 0.5] Go Down through platform
  (:Pressed
    (Utilities|FlowControl|Gate true
      (:Exit
        (Collision|SetCollisionEnabled (Variables|Default|GetPlatform) "NoCollision")))))

(fn ConstructionScript)