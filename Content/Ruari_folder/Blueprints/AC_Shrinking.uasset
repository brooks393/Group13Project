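; AC_Shrinking is a component that shrinks or regrows the player in response to Shrink and Growth Potion item actions.
; It finds the level's BP_ShrinkTimeline actor at BeginPlay and plays or reverses its shrink on the player character, with a sound.
; Growth first line-traces upward from the player for headroom and leaves them small if blocked.
; It tracks the result in PlayerIsSmall.
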(event EventBeginPlay
  ;[0.15 0.15 0.15 0.5] Get Timeline
  (bind _returnvalue (Actor|GetActorOfClass "/Game/Ruari_folder/Blueprints/BP_ShrinkTimeline.BP_ShrinkTimeline_C"))
  (Variables|Default|SetTimeline _returnvalue))

(event EventBindMinigameAction
  (params (LocationlessItem? :type E_LocationlessItems%20Enum :default "NewEnumerator2"))
  (bind _returnvalue (Game|GetPlayerCharacter 0))
  (bind _timeline (Variables|Default|GetTimeline))
  (bind _returnvalue_2 (Transformation|GetActorLocation _returnvalue))
  (switch Utilities|FlowControl|Switch|SwitchonE_LocationlessItems LocationlessItem?
    (:NewEnumerator0
      ;[0.15 0.15 0.15 0.5] Growing
      (bind _returnvalue_3 (Collision|LineTraceByChannel _returnvalue_2 (+ _returnvalue_2 (* (Transformation|GetActorUpVector (Game|GetPlayerCharacter 0)) 1.4e+02)) "TraceTypeQuery1" false (Utilities|Array|MakeArray (Game|GetPlayerCharacter 0)) "ForDuration"))
      (if _returnvalue_3
        (Variables|Default|SetPlayerIsSmall? true)
        (else
          (Default|ReverseShrink (Variables|Default|GetTimeline) (Game|GetPlayerCharacter 0))
          (Variables|Default|SetPlayerIsSmall? false)
          (Audio|PlaySound2D "/Game/Rey/Audio/SW_Grow.SW_Grow" 1.0 1.0 0.0 0 0))))
    (:NewEnumerator1
      ;[0.15 0.15 0.15 0.5] Shrinking
      (Utilities|IsValid _timeline
        (:Is%20Valid
          (Default|PlayShrink _timeline (Game|GetPlayerCharacter 0))
          (Variables|Default|SetPlayerIsSmall? true)
          (Audio|PlaySound2D "/Game/Rey/Audio/SW_Shrink.SW_Shrink" 1.0 1.0 0.0 0 0))
        (:Is%20Not%20Valid
          (Development|PrintString "Shrink Fail")
          (Variables|Default|SetPlayerIsSmall? false))))))

(fn GetContextualUseText
  (return ""))

(fn GetIsMinigame
  (return "NewEnumerator0"))