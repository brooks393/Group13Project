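; Analog clock actor that starts at the computer's current time and serves as a hand-winding minigame.
; Using it starts a one-second looping timer that advances the hands, switches the view to the clock, shows the cursor and hides the player mesh.
; GetObjectUnderMouse toggles winding, which stops the timer and turns the minute hand toward the mouse through next-tick recursion.
; The hour hand follows by range mapping, tracking hour rollovers.
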(event OnComponentBeginOverlap(Box)
  (params (OverlappedComponent :type Primitive%20Component%20Object%20Reference) (OtherActor :type Actor%20Object%20Reference) (OtherComp :type Primitive%20Component%20Object%20Reference) (OtherBodyIndex :type Integer) (bFromSweep :type Boolean) (SweepResult :type Hit%20Result%20Structure%20%28by%20ref%29))
  ;[0.15 0.15 0.15 0.5] Stop clock hands
)

(event OnComponentEndOverlap(Box)
  (params (OverlappedComponent :type Primitive%20Component%20Object%20Reference) (OtherActor :type Actor%20Object%20Reference) (OtherComp :type Primitive%20Component%20Object%20Reference) (OtherBodyIndex :type Integer))
  ;[0.15 0.15 0.15 0.5] Restart clock hands
)

(event Custom|GetObjectUnderMouse
  ;[0.15 0.15 0.15 0.5] Toggle winding on left click
  (Utilities|FlowControl|FlipFlop
    (:A
      (Variables|Default|SetWindingClock? true)
      (CallFunction|StopClock)
      (CallFunction|DoRotateHandtoMouse))
    (:B
      (Variables|Default|SetWindingClock? false)
      (CallFunction|RestartClock))))

(event Custom|OnRotateSecondHand
  ;[0.15 0.15 0.15 0.5] Set correct clock hand rotation
  (CallFunction|IncrementSecondHand)
  (CallFunction|IncrementMinuteHand)
  (if (Math|Float|NearlyEqual(Float) (.Remainder (Math|Float|Division(WholeandRemainder) (.roll (Transformation|GetWorldRotation (Variables|Default|GetMinuteHand))) 9e+01)) 0.0 0.1)
    (Utilities|FlowControl|DoOnce false :!label _label
      (:Completed
        (CallFunction|IncrementHourHand)))
    (else
      (goto _label Reset))))

(event Custom|StopClock
  ;[0.15 0.15 0.15 0.5] Stop clock hands
  (Utilities|Time|ClearandInvalidateTimerbyHandle (Variables|Default|GetSecondHandTimer)))

(event Custom|RestartClock
  ;[0.15 0.15 0.15 0.5] Set correct clock hand rotation
  (bind _returnvalue (Utilities|Time|SetTimerbyEvent (delegate Custom|OnRotateSecondHand) 1.0 true))
  (Variables|Default|SetSecondHandTimer _returnvalue))

(event Custom|DoRotateHandToMouse
  (bind _returnvalue (Utilities|GetRotationtoMouseLocation))
  (bind _currenthour (Variables|Default|GetCurrentHour))
  (bind (_roll _pitch _yaw) (Math|Rotator|BreakRotator _returnvalue))
  (bind _returnvalue_2 (* _currenthour 30))
  ;[0.15 0.15 0.15 0.5] Update Hands Rotation
  (if (Variables|Default|GetWindingClock?)
    (Transformation|SetRelativeRotation (Variables|Default|GetMinuteHand) _returnvalue false false)
    (Variables|Default|SetMinuteHandRotation _returnvalue)
    (Variables|Default|SetCurrent%20X (.Roll (Math|Rotator|BreakRotator (Variables|Default|GetMinuteHandRotation))))
    (if (and (> (Variables|Default|GetCurrent%20X) 0.0) (< (Variables|Default|GetLast%20X) 0.0))
      (Utilities|IncrementCurrentHour))
    (Transformation|SetRelativeRotation (Variables|Default|GetHourHand) (Math|Rotator|MakeRotator (Math|Float|MapRangeClamped _roll 1.8e+02 -1.8e+02 (Math|Conversions|ToFloat(Integer) _returnvalue_2) (Math|Conversions|ToFloat(Integer) (- _returnvalue_2 30))) _pitch _yaw) false false)
    (Variables|Default|SetLast%20X (.roll (Variables|Default|GetMinuteHandRotation)))
    (Utilities|FlowControl|DelayUntilNextTick)
    (CallFunction|DoRotateHandtoMouse)))

(event EventBeginPlay
  (bind _returnvalue (Math|DateTime|Now))
  ;[0.15 0.15 0.15 0.5] Set correct clock hand rotation
  ;;[0.15 0.15 0.15 0.5] Set initial time based on IRL (computer) clock time
  (Variables|Default|SetCurrentHour (.hour _returnvalue))
  (CallFunction|SetHourHand (.hour _returnvalue) (.minute _returnvalue))
  (CallFunction|SetMinute/SecondHand (.minute _returnvalue) (Variables|Default|GetMinuteHand))
  (CallFunction|SetMinute/SecondHand (.second _returnvalue) (Variables|Default|GetSecondHand)))

(event EventItemUsed
  (bind _returnvalue (Game|GetPlayerController 0))
  ;[0.15 0.15 0.15 0.5] Use minigame camera, hide player model, set correct input controls
  (CallFunction|RestartClock)
  (bind _returnvalue_2 (Actor|GetActorOfClass "/Game/Rey/BP_Rey_ThirdPersonCharacter.BP_Rey_ThirdPersonCharacter_C"))
  (Variables|/Game/Rey/CharacterComponents/AC_InventoryComponent.AC_InventoryComponent_C|SetIsInMinigame? (Variables|/Game/Rey/BP_Rey_ThirdPersonCharacter.BP_Rey_ThirdPersonCharacter_C|GetAC_InventoryComponent _returnvalue_2) true)
  (Game|Player|SetViewTargetwithBlend (Game|GetPlayerController 0) self 0.5 "VTBlend_Cubic" 0.0 false)
  (Default|OnCloseInventory (Actor|GetComponentbyClass (Game|GetPlayerCharacter 0) "/Game/Rey/CharacterComponents/AC_InventoryComponent.AC_InventoryComponent_C"))
  (Input|SetInputModeGameandUI _returnvalue 0 "DoNotLock" false true)
  (Variables|/Script/Engine.PlayerController|SetbShowMouseCursor _returnvalue true)
  (Rendering|SetVisibility (Variables|/Script/Engine.Character|GetMesh (Game|GetPlayerCharacter 0)) false true))

(fn ConstructionScript)

(fn SetHourHand
  (params (Hour :type Integer) (Minute :type Integer))
  (LocalVariables|SetHourValue Hour)
  (LocalVariables|SetMinuteValue Minute)
  (if (> (LocalVariables|GetHourValue) 12)
    (Transformation|SetWorldRotation (Variables|Default|GetHourHand) (Math|Rotator|MakeRotator (Math|Conversions|ToFloat(Integer) (* (- (LocalVariables|GetHourValue) 12) 30)) 0.0 0.0) false false)
    (else
      (Transformation|SetWorldRotation (Variables|Default|GetHourHand) (Math|Rotator|MakeRotator (Math|Conversions|ToFloat(Integer) (* (LocalVariables|GetHourValue) 30)) 0.0 0.0) false false)))
  (if (== (/ (LocalVariables|GetMinuteValue) 15) 0)
    (Transformation|AddWorldRotation (Variables|Default|GetHourHand) (Math|Rotator|MakeRotator (Math|Conversions|ToFloat(Integer) (/ (LocalVariables|GetMinuteValue) 15)) 0.0 0.0) false false)))

(fn SetMinute/SecondHand
  (params (A :type Integer) (Target :type Scene%20Component%20Object%20Reference))
  (Transformation|SetWorldRotation Target (Math|Rotator|MakeRotator (Math|Conversions|ToFloat(Integer) (* A 6)) 0.0 0.0) false false))

(fn IncrementSecondHand
  (bind _secondhand (Variables|Default|GetSecondHand))
  (Transformation|AddLocalRotation _secondhand "0.000000,0.000000,6.000000" false false)
  (if (>= (.roll (Transformation|GetWorldRotation _secondhand)) 3.6e+02)
    (Transformation|SetWorldRotation (Variables|Default|GetSecondHand) "0, 0, 0" false false)))

(fn IncrementMinuteHand
  (if (Math|Float|NearlyEqual(Float) (.Remainder (Math|Float|Division(WholeandRemainder) (.roll (Transformation|GetWorldRotation (Variables|Default|GetSecondHand))) 3.6e+02)) 0.0 0.1)
    (Transformation|AddLocalRotation (Variables|Default|GetMinuteHand) "0.000000,0.000000,6.000000" false false)))

(fn IncrementHourHand
  (Transformation|AddLocalRotation (Variables|Default|GetHourHand) "0.000000,0.000000,7.500000" false false))