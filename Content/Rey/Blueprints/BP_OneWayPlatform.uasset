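; A one-way platform that the BrandonPerson character can pass through and then stand on.
; Overlapping PassthroughZone disables the static mesh's collision.
; A SafeZone trigger tracks whether the character is above the platform, and two booleans combine both zones' states.
; Collision is restored only when the character is in SafeZone and outside PassthroughZone, checked on SafeZone entry and PassthroughZone exit.
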(event OnComponentBeginOverlap(PassthroughZone)
  (params (OverlappedComponent :type Primitive%20Component%20Object%20Reference) (OtherActor :type Actor%20Object%20Reference) (OtherComp :type Primitive%20Component%20Object%20Reference) (OtherBodyIndex :type Integer) (bFromSweep :type Boolean) (SweepResult :type Hit%20Result%20Structure%20%28by%20ref%29))
  (if (== (Utilities|GetClass OtherActor) "/Game/ThirdPerson/Blueprints/BrandonPerson.BrandonPerson_C")
    (Variables|Default|SetIsCharacterInPlatform? true)
    (Collision|SetCollisionEnabled (Variables|Default|GetStaticMesh) "NoCollision")))

(event OnComponentBeginOverlap(SafeZone)
  (params (OverlappedComponent :type Primitive%20Component%20Object%20Reference) (OtherActor :type Actor%20Object%20Reference) (OtherComp :type Primitive%20Component%20Object%20Reference) (OtherBodyIndex :type Integer) (bFromSweep :type Boolean) (SweepResult :type Hit%20Result%20Structure%20%28by%20ref%29))
  (if (== (Utilities|GetClass OtherActor) "/Game/ThirdPerson/Blueprints/BrandonPerson.BrandonPerson_C")
    (Variables|Default|SetIsCharacterAbovePlatform? true)
    (if (not (Variables|Default|GetIsCharacterInPlatform?))
      (Collision|SetCollisionEnabled (Variables|Default|GetStaticMesh) "QueryAndPhysics"))))

(event OnComponentEndOverlap(PassthroughZone)
  (params (OverlappedComponent :type Primitive%20Component%20Object%20Reference) (OtherActor :type Actor%20Object%20Reference) (OtherComp :type Primitive%20Component%20Object%20Reference) (OtherBodyIndex :type Integer))
  (if (== (Utilities|GetClass OtherActor) "/Game/ThirdPerson/Blueprints/BrandonPerson.BrandonPerson_C")
    (Variables|Default|SetIsCharacterInPlatform? false)
    (if (Variables|Default|GetIsCharacterAbovePlatform?)
      (Collision|SetCollisionEnabled (Variables|Default|GetStaticMesh) "QueryAndPhysics"))))

(event OnComponentEndOverlap(SafeZone)
  (params (OverlappedComponent :type Primitive%20Component%20Object%20Reference) (OtherActor :type Actor%20Object%20Reference) (OtherComp :type Primitive%20Component%20Object%20Reference) (OtherBodyIndex :type Integer))
  (if (== (Utilities|GetClass OtherActor) "/Game/ThirdPerson/Blueprints/BrandonPerson.BrandonPerson_C")
    (Variables|Default|SetIsCharacterAbovePlatform? false)))

(event EventBeginPlay)

(event Collision|EventActorBeginOverlap
  (params (OtherActor :type Actor%20Object%20Reference)))

(event EventTick
  (params (DeltaSeconds :type Float%20%28single-precision%29)))

(fn ConstructionScript)