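; BP_InteractWithApple is an interactable apple that plays a 2D crunch sound when used.
; The ItemUsed event triggers the sound and does nothing else.
; Two getter functions expose its contextual use text and minigame flag.
; BeginPlay, overlap and Tick are disabled stubs, and the construction script only calls its parent.
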(event EventBeginPlay
  (|CallParentFunction) ; This node is disabled and will not be called.\nDrag off pins to build functionality.
)

(event Collision|EventActorBeginOverlap
  (params (OtherActor :type Actor%20Object%20Reference))
  (|CallParentFunction OtherActor) ; This node is disabled and will not be called.\nDrag off pins to build functionality.
)

(event EventTick
  (params (DeltaSeconds :type Float%20%28single-precision%29))
  (|CallParentFunction DeltaSeconds) ; This node is disabled and will not be called.\nDrag off pins to build functionality.
)

(event EventItemUsed
  ;[0.15 0.15 0.15 0.5] test
  (Audio|PlaySound2D "/Game/Rey/TempTestingDeleteLater/SW_Crunch.SW_Crunch" 1.0 1.0 0.0 0 0))

(fn ConstructionScript
  (|CallParentFunction))

(fn GetContextualUseText
  (return (Variables|Default|GetContextualUseText)))

(fn GetIsMinigame
  (return (Variables|Default|GetIsMinigame?)))