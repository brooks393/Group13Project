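; Pop-up component that rotates nearby objects as the player approaches, like pieces tipping up in a pop-up book.
; Every tick it runs a zero-length multi-sphere trace for configured object types around the first player character.
; Each blocking hit actor's relative roll is mapped from player distance, reaching 90 degrees up close, while pitch and yaw are copied from its world rotation.
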(event EventTick
  (params (DeltaSeconds :type Float%20%28single-precision%29))
  (bind _returnvalue (Game|GetPlayerCharacter 0))
  (bind _returnvalue_2 (Transformation|GetActorLocation _returnvalue))
  (if (Utilities|IsValid _returnvalue)
    (bind _outhits (Collision|MultiSphereTraceForObjects _returnvalue_2 _returnvalue_2 5e+02 (Variables|Default|GetObject%20Types) false 0 "None" true "(R=1.000000,G=0.000000,B=0.000000,A=1.000000)" "(R=0.000000,G=1.000000,B=0.000000,A=1.000000)" 1.0))
    (for _array_element _outhits
      (if (.bBlockingHit (Collision|BreakHitResult _array_element))
        (Transformation|SetActorRelativeRotation (.HitActor (Collision|BreakHitResult _array_element)) (Math|Rotator|MakeRotator (Math|Float|MapRangeClamped (Transformation|GetDistanceTo (Game|GetPlayerCharacter 0) (.HitActor (Collision|BreakHitResult _array_element))) 5e+02 1.5e+02 0.0 9e+01) (.pitch (Transformation|GetActorRotation (.HitActor (Collision|BreakHitResult _array_element)))) (.yaw (Transformation|GetActorRotation (.HitActor (Collision|BreakHitResult _array_element))))))))))