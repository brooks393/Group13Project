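; Actor component for the Rey character that handles pausing and unpausing the game through a pause menu widget.
; On BeginPlay it creates WBP_PauseMenu with a reference to itself and adds it to the viewport collapsed.
; The IA_PauseMenu input pauses the game, shows the menu and switches to UI-only input with a visible cursor.
; UnpauseGame reverses this, restoring game-only input and hiding the menu and cursor.
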(event Input|EnhancedActionEvents|EnhancedInputActionIA_PauseMenu
  (params (ActionValue :type Boolean) (ElapsedSeconds :type Float%20%28double-precision%29) (TriggeredSeconds :type Float%20%28double-precision%29) (InputAction :type Input%20Action%20Object%20Reference :default "/Game/Input/Actions/IA_PauseMenu.IA_PauseMenu"))
  (bind _returnvalue (Game|GetPlayerController 0))
  (:Started
    (Game|SetGamePaused true)
    (Widget|SetVisibility (Variables|Default|GetPauseMenuWidget) "Visible")
    (Input|SetInputModeUIOnly _returnvalue 0 "DoNotLock" true)
    (Variables|/Script/Engine.PlayerController|SetbShowMouseCursor _returnvalue true)))

(event EventBeginPlay
  (bind _returnvalue (UserInterface|CreateWidget "/Game/Rey/Widgets/WBP_PauseMenu.WBP_PauseMenu_C" 0 self))
  (bind _output_get (Variables|Default|SetPauseMenuWidget _returnvalue))
  (Widget|SetVisibility _output_get "Collapsed")
  (UserInterface|Viewport|AddtoViewport (Variables|Default|GetPauseMenuWidget) 0))

(fn UnpauseGame
  (bind _returnvalue (Game|GetPlayerController 0))
  ;[0.15 0.15 0.15 0.5] Unpause Game
  (Game|SetGamePaused false)
  (Widget|SetVisibility (Variables|Default|GetPauseMenuWidget) "Collapsed")
  (Input|SetInputModeGameOnly _returnvalue true)
  (Variables|/Script/Engine.PlayerController|SetbShowMouseCursor _returnvalue false))