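; Actor component that opens and closes the game's pause menu.
; Pressing P pauses the game, creates a WBP_PauseMenu widget holding a reference to this component, and switches to UI-only input with the cursor shown.
; UnpauseGame reverses this by resuming the game, removing the widget and restoring game-only input with the cursor hidden.
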(event EventBeginPlay)

(event EventTick
  (params (DeltaSeconds :type Float%20%28single-precision%29)))

(event Input|KeyboardEvents|P
  (params (Key :type Key%20Structure :default "None"))
  (bind _returnvalue (Game|GetPlayerController 0))
  (:Pressed
    (Game|SetGamePaused true)
    (bind _returnvalue_2 (UserInterface|CreateWidget "/Game/Rey/Widgets/WBP_PauseMenu.WBP_PauseMenu_C" 0 self))
    (bind _output_get (Variables|Default|SetPauseMenuWidget _returnvalue_2))
    (UserInterface|Viewport|AddtoViewport _output_get 0)
    (Input|SetInputModeUIOnly _returnvalue 0 "DoNotLock" true)
    (Variables|/Script/Engine.PlayerController|SetbShowMouseCursor _returnvalue true)))

(fn UnpauseGame
  (bind _returnvalue (Game|GetPlayerController 0))
  (Game|SetGamePaused false)
  (Widget|RemovefromParent (Variables|Default|GetPauseMenuWidget))
  (Input|SetInputModeGameOnly _returnvalue true)
  (Variables|/Script/Engine.PlayerController|SetbShowMouseCursor _returnvalue false))