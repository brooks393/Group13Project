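; Player inventory component that picks up nearby items and shows them in a WBP_Inventory widget, created hidden on BeginPlay.
; E toggles the widget, switching input mode and mouse cursor.
; Left click sphere-traces at the character's feet for the first BPI_PickUp actor, adds its BP_Item data to HeldItems if new, destroys it and reloads the widget.
; During a minigame, left click instead calls GetObjectUnderMouse on BP_Clock.
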(event Custom|BreakObjectSearch
  ;[0 0 0 0.5] Object Pickup
  ;;[0.07057 0.136 0.15 0.5] Only retrieve objects that implement BPI_PickUp
  (Utilities|Array|ForEachLoopwithBreak (stale Input|MouseEvents|LeftMouseButton _outhits)) ; enters at Break
)

(event Custom|OnCloseInventory
  (bind _returnvalue (Game|GetPlayerController 0))
  ;[0 0 0 0.5] Toggle open/close inventory
  (Widget|SetVisibility (Variables|Default|GetInventoryWidget) "Collapsed")
  (Input|SetInputModeGameOnly _returnvalue false)
  (Variables|/Script/Engine.PlayerController|SetbShowMouseCursor _returnvalue false)
  (Default|CloseInventoryChildren (Variables|Default|GetInventoryWidget)))

(event EventBeginPlay
  ;[0 0 0 0.5] Create inventory widget, make invisible, add to player viewport
  (bind _returnvalue (UserInterface|CreateWidget "/Game/Rey/Widgets/WBP_Inventory.WBP_Inventory_C"))
  (bind _output_get (Variables|Default|SetInventoryWidget _returnvalue))
  (Widget|SetVisibility _output_get "Collapsed")
  (UserInterface|Viewport|AddtoViewport (Variables|Default|GetInventoryWidget) 0)
  (Default|LoadInventory (Variables|Default|GetInventoryWidget) self))

(event Input|MouseEvents|LeftMouseButton
  (params (Key :type Key%20Structure :default "None"))
  (bind _returnvalue (Game|GetPlayerCharacter 0))
  (bind _returnvalue_2 (Transformation|GetActorLocation _returnvalue))
  (bind _returnvalue_3 (- _returnvalue_2 "0.000000,0.000000,65.000000"))
  (:Pressed
    (if (Variables|Default|GetIsInMinigame?)
      (bind _returnvalue_4 (Actor|GetActorOfClass "/Game/Rey/Blueprints/BP_Clock.BP_Clock_C"))
      (Default|GetObjectUnderMouse _returnvalue_4)
      (else
        ;[0 0 0 0.5] Object Pickup
        ;;[0.15 0.15 0.15 0.5] Run trace
        ;;;[0.15 0.05382 0.05812 0.5] Clear prev. data (if any)
        (Variables|Default|SetHit%20Actor 0)
        (Variables|Default|SetInventory%20Item%20Data "")
        (bind _outhits (Collision|MultiSphereTraceByChannel _returnvalue_3 _returnvalue_3 1e+02 "TraceTypeQuery1" false 0 "ForDuration" true "(R=0.027293,G=0.001422,B=1.000000,A=1.000000)" "(R=1.000000,G=0.880102,B=0.000000,A=1.000000)"))
        ;;[0.07057 0.136 0.15 0.5] Only retrieve objects that implement BPI_PickUp
        (bind _array_element (Utilities|Array|ForEachLoopwithBreak _outhits)
          (:LoopBody
            (bind _output_get (Variables|Default|SetHit%20Actor (.HitActor (Collision|BreakHitResult _array_element))))
            (if (Utilities|DoesObjectImplementInterface _output_get "/Game/Rey/BlueprintInterfaces/BPI_PickUp.BPI_PickUp_C")
              (CallFunction|BreakObjectSearch)
              ;;[0.07813 0.08424 0.15 0.5] (Re)load inventory widget with item data and destroy actor
              (bind _asbp_item (Utilities|Casting|CastToBP_Item (Variables|Default|GetHit%20Actor)))
              (bind _output_get_2 (Variables|Default|SetInventory%20Item%20Data (Variables|/Game/Rey/Blueprints/BP_Item.BP_Item_C|GetInventoryItemData _asbp_item)))
              (if (not (Utilities|Array|ContainsItem (Variables|Default|GetHeldItems) _output_get_2))
                (Utilities|Array|Add (Variables|Default|GetHeldItems) (Variables|Default|GetInventory%20Item%20Data))
                (Actor|DestroyActor (Variables|Default|GetHit%20Actor))
                (Default|LoadInventory (Variables|Default|GetInventoryWidget) self)))))))))

(event Input|KeyboardEvents|E
  (params (Key :type Key%20Structure :default "None"))
  (bind _returnvalue (Game|GetPlayerController 0))
  ;[0 0 0 0.5] Toggle open/close inventory
  (:Pressed
    (if (Widget|IsVisible (Variables|Default|GetInventoryWidget))
      (Widget|SetVisibility (Variables|Default|GetInventoryWidget) "Collapsed")
      (Input|SetInputModeGameOnly _returnvalue false)
      (Variables|/Script/Engine.PlayerController|SetbShowMouseCursor _returnvalue false)
      (Default|CloseInventoryChildren (Variables|Default|GetInventoryWidget))
      (else
        (Widget|SetVisibility (Variables|Default|GetInventoryWidget) "Visible")
        (Input|SetInputModeGameandUI _returnvalue 0 "DoNotLock" true false)
        (Variables|/Script/Engine.PlayerController|SetbShowMouseCursor _returnvalue true)))))