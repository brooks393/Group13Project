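; Main camera pawn for a mouse-driven book selection screen, showing an animated art-block explanation widget on begin play.
; Each Tick traces under the cursor, pushes in every BP_Book and messages the hovered interactable, an approach marked for optimisation.
; IA_Interact gets the clicked book, removes the widget, then either fires its teleporter or moves and possesses BrandonPerson with the book's level camera.
; Three older hover attempts remain disconnected.
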(event Input|EnhancedActionEvents|EnhancedInputActionIA_Interact
  (params (ActionValue :type Boolean) (ElapsedSeconds :type Float%20%28double-precision%29) (TriggeredSeconds :type Float%20%28double-precision%29) (InputAction :type Input%20Action%20Object%20Reference :default "/Game/Input/Actions/IA_Interact.IA_Interact"))
  (bind _returnvalue (Game|GetPlayerController 0))
  (bind _returnvalue_2 (Game|GetPlayerController 0))
  (bind _artblockwidget (Variables|Default|GetArtBlockWidget))
  (bind _hitresult (Game|Player|GetHitResultUnderCursorbyChannel _returnvalue_2 "TraceTypeQuery1" true))
  (bind _hitactor (Collision|BreakHitResult _hitresult))
  ;[0 1 0] On Enhanced Input Interact -
  (:Started
    (Variables|Default|SetHit%20Actor _hitactor)
    (if (Utilities|DoesObjectImplementInterface _hitactor "/Game/Brandon/Interfaces/BI_GetBook.BI_GetBook_C")
      (bind _selectedbook (Class|BIGetBook|GetBook(Message) _hitactor))
      (bind _output_get (Variables|Default|SetBookSelected _selectedbook))
      (if (Variables|/Game/Brandon/Bookcase/Book/BP_Book.BP_Book_C|GetUseTeleporter? _selectedbook)
        (Variables|Default|SetCurrTP%20Location (Variables|/Game/Brandon/Bookcase/Book/BP_Book.BP_Book_C|GetTeleport _selectedbook))
        (Default|TeleporttoHere :self (Variables|Default|GetCurrTP%20Location) :USeTeleportoer true)
        (Variables|/Game/Brandon/Bookcase/Book/BP_Book.BP_Book_C|SetUseTeleporter? _output_get false)
        (Widget|RemovefromParent _artblockwidget)
        (else
          (bind _returnvalue_3 (Actor|GetActorOfClass "/Game/ThirdPerson/Blueprints/BrandonPerson.BrandonPerson_C"))
          (Transformation|SetActorTransform _returnvalue_3 (Math|Transform|MakeTransform (.location (Variables|/Game/Brandon/Bookcase/Book/BP_Book.BP_Book_C|GetBooksPlayerPosition _selectedbook)) "0, 0, 0" (.scale (Variables|/Game/Brandon/Bookcase/Book/BP_Book.BP_Book_C|GetBooksPlayerPosition _selectedbook))))
          (Widget|RemovefromParent _artblockwidget)
          (Pawn|Possess _returnvalue _returnvalue_3)
          (Variables|/Script/Engine.PlayerController|SetbShowMouseCursor _returnvalue false)
          (Game|Player|SetViewTargetwithBlend (Game|GetPlayerController 0) (Variables|/Game/Brandon/Bookcase/Book/BP_Book.BP_Book_C|GetLevelCamera (Variables|Default|GetBookSelected)) 0.0 "VTBlend_Linear" 0.0 false))))))

(event EventBeginPlay
  (bind _returnvalue (Game|GetPlayerController 0))
  ;[0 1 0] On Event Begin Play, sets input mode to game and UI and adds the Widget Blueprint to players viewport and plays the widget animation
  (Variables|/Script/Engine.PlayerController|SetbShowMouseCursor _returnvalue true)
  (Input|SetInputModeGameandUI _returnvalue 0 "DoNotLock" true false)
  (bind _returnvalue_2 (UserInterface|CreateWidget "/Game/Brandon/UI/WBP_ArtBlockExplanation.WBP_ArtBlockExplanation_C" (Game|GetPlayerController 0)))
  (Variables|Default|SetArtBlockWidget _returnvalue_2)
  (UserInterface|Viewport|AddtoViewport _returnvalue_2 0)
  (UserInterface|Animation|PlayAnimation _returnvalue_2 (Variables|/Game/Brandon/UI/WBP_ArtBlockExplanation.WBP_ArtBlockExplanation_C|GetArtUnblockStarter _returnvalue_2) 0.0 1 "Forward" 1.0 false))

(event EventTick
  (params (DeltaSeconds :type Float%20%28single-precision%29))
  (bind _returnvalue (Game|GetPlayerController 0))
  (bind _hitresult (Game|Player|GetHitResultUnderCursorbyChannel _returnvalue "TraceTypeQuery1" true))
  (bind _hitactor (Collision|BreakHitResult _hitresult))
  (if (Utilities|DoesObjectImplementInterface _hitactor "/Game/Brandon/Interfaces/BPI_Interact.BPI_Interact_C")
    (Variables|Default|SetHit%20Actor _hitactor)
    ;[1 0 0] Optimsie
    (bind _outactors (Actor|GetAllActorsOfClass "/Game/Brandon/Bookcase/Book/BP_Book.BP_Book_C"))
    (for _array_element _outactors
      (Default|ForcePushin _array_element))
    (Variables|Default|SetCurrentHoveredBook (Variables|Default|GetHit%20Actor))
    (Class|BPIInteract|INteract(Message) (Variables|Default|GetCurrentHoveredBook) 0 true)))

(fn ConstructionScript)