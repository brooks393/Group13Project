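; BP_Book is an interactable book, filed under Bookcase, that tilts and slides out when pulled and returns when pushed.
; INteract, ignored while the book moves, either adds an outline overlay and pulls, or removes it and pushes, tracking the state in HadMoved.
; One timeline drives clamped relative offset and roll on the Scene component, playing forward or reversed.
; ForcePushIn clears the outline and reverses it without the movement check.
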(event Custom|Pull
  (bind _newtrack_0 (Timeline|Timeline Play)
    (:Update
      (Transformation|SetRelativeLocation (Variables|Default|GetScene) (Math|Vector|MakeVector 0.0 (Math|Float|Clamp(Float) (* _newtrack_0 2e+01) 0.0 5.0) 0.0) false false)
      (Transformation|SetRelativeRotation (Variables|Default|GetScene) (Math|Rotator|MakeRotator (Math|Float|Clamp(Float) (* _newtrack_0 2e+01) 0.0 4e+01) 0.0 0.0) false false)
      (Variables|Default|SetisMoving true))
    (:Finished
      (Variables|Default|SetisMoving false))))

(event Custom|Push
  (bind _newtrack_0 (Timeline|Timeline Reverse)
    (:Update
      (Transformation|SetRelativeLocation (Variables|Default|GetScene) (Math|Vector|MakeVector 0.0 (Math|Float|Clamp(Float) (* _newtrack_0 2e+01) 0.0 5.0) 0.0) false false)
      (Transformation|SetRelativeRotation (Variables|Default|GetScene) (Math|Rotator|MakeRotator (Math|Float|Clamp(Float) (* _newtrack_0 2e+01) 0.0 4e+01) 0.0 0.0) false false)
      (Variables|Default|SetisMoving true))
    (:Finished
      (Variables|Default|SetisMoving false))))

(event Custom|Remove%20Outlin
  (Rendering|Material|SetOverlayMaterial (Variables|Default|GetCube) 0 :!class /Script/Engine.MeshComponent)
  (Rendering|Material|SetOverlayMaterial (Variables|Default|GetCylinder) 0 :!class /Script/Engine.MeshComponent))

(event Custom|SetOutline
  (Rendering|Material|SetOverlayMaterial (Variables|Default|GetCube) "/Game/Brandon/Outline.Outline" :!class /Script/Engine.MeshComponent)
  (Rendering|Material|SetOverlayMaterial (Variables|Default|GetCylinder) "/Game/Brandon/Outline.Outline" :!class /Script/Engine.MeshComponent))

(event Custom|ForcePushIn
  (CallFunction|RemoveOutlin)
  (CallFunction|Push))

(event EventBeginPlay
  (Variables|Default|SetWorldLocation (Variables|/Script/Engine.SceneComponent|GetRelativeLocation (Variables|Default|GetScene))))

(event Collision|EventActorBeginOverlap
  (params (OtherActor :type Actor%20Object%20Reference)))

(event EventINteract
  (params (Interact :type Character%20Object%20Reference) (IsStarting :type Boolean))
  (if (not (Variables|Default|GetisMoving))
    (if IsStarting
      (CallFunction|SetOutline)
      (Variables|Default|SethadMoved true)
      (CallFunction|Pull)
      (else
        (CallFunction|RemoveOutlin)
        (Variables|Default|SethadMoved false)
        (CallFunction|Push)))))

(event MouseInput|EventActorBeginCursorOver
  (Development|PrintString "Hello"))

(fn ConstructionScript)