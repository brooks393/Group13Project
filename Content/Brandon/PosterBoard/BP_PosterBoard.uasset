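; BP_PosterBoard is a board actor that displays a poster for each of three levels according to the ending type reached.
; The construction script collects the Level1, Level2 and Level3 scene components into an array of poster slots.
; AddPoster takes a level number and ending type, then SpawningPoster spawns a BP_Poster at that slot's world transform and sets its material from the ending type.
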(event Custom|AddPoster
  (params (LevelInt :type Integer) (EndingType :type Integer))
  (switch int LevelInt
    (:1
      (CallFunction|SpawningPoster 1 EndingType))
    (:2
      (CallFunction|SpawningPoster 2 EndingType))
    (:3
      (CallFunction|SpawningPoster 3 EndingType))))

(event EventBeginPlay)

(event Collision|EventActorBeginOverlap
  (params (OtherActor :type Actor%20Object%20Reference)))

(event EventTick
  (params (DeltaSeconds :type Float%20%28single-precision%29)))

(fn ConstructionScript
  (bind _arrayofposterscenes (Variables|Default|GetArrayOfPosterScenes))
  (Utilities|Array|Add _arrayofposterscenes (Variables|Default|GetLevel1))
  (Utilities|Array|Add _arrayofposterscenes (Variables|Default|GetLevel2))
  (Utilities|Array|Add _arrayofposterscenes (Variables|Default|GetLevel3)))

(fn SpawningPoster
  (params (Level :type Integer) (EndingType :type Integer))
  (bind _returnvalue (Game|SpawnActorfromClass "/Game/Brandon/PosterBoard/BP_Poster.BP_Poster_C" (Transformation|GetWorldTransform (Utilities|Array|Get(acopy) (Variables|Default|GetArrayOfPosterScenes) (- Level 1))) "AlwaysSpawn" "MultiplyWithRoot" 0 0 0 0))
  (Default|SetMaterial _returnvalue 0 0 EndingType))