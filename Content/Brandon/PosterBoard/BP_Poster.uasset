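; BP_Poster is a poster whose Cube mesh shows a material chosen by ending type and level.
; Its SetMaterial event picks the good or bad ending material array from the EndingType boolean and applies the entry matching the 1-based LevelIndex to slot 0.
; It finds that entry by looping over the array rather than indexing it.
; The event's GoodEndingMat and BadEndingMat inputs are unused.
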(event Custom|SetMaterial
  (params (GoodEndingMat :type Array%20of%20Material%20Object%20References) (BadEndingMat :type Array%20of%20Material%20Object%20References) (EndingType :type Boolean) (LevelIndex :type Integer))
  (if EndingType
    (for (_array_element _array_index) (Variables|Default|GetGoodEndingPosterMaterial)
      (if (== (+ _array_index 1) LevelIndex)
        (Rendering|Material|SetMaterial (Variables|Default|GetCube) 0 _array_element)))
    (else
      (for (_array_element_2 _array_index_2) (Variables|Default|GetBadEndingPosterMaterial)
        (if (== (+ _array_index_2 1) LevelIndex)
          (Rendering|Material|SetMaterial (Variables|Default|GetCube) 0 _array_element_2))))))

(fn ConstructionScript)