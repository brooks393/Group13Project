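; BP_Wires is an interactable wire prop for a minigame that gets cut when the Interact event fires.
; The construction script sets the intact wire mesh, its scale and its material.
; Interacting swaps in the cut mesh, then finds the BP_PosterBoard actor by class and adds a level 2 poster flagged as not the good ending.
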(event EventBeginPlay)

(event Collision|EventActorBeginOverlap
  (params (OtherActor :type Actor%20Object%20Reference)))

(event EventTick
  (params (DeltaSeconds :type Float%20%28single-precision%29)))

(event EventINteract
  (params (Interact :type Character%20Object%20Reference) (IsStarting :type Boolean) (vent :type BP%20Vent%20Object%20Reference))
  (Components|StaticMesh|SetStaticMesh (Variables|Default|GetFull_Wire) (Variables|Default|GetCutWireMesh))
  (bind _returnvalue (Actor|GetActorOfClass "/Game/Brandon/PosterBoard/BP_PosterBoard.BP_PosterBoard_C"))
  (Variables|Default|SetPosterBoard _returnvalue)
  (Default|AddPoster (Variables|Default|GetPosterBoard) false "0, 0, 0" 2))

(fn ConstructionScript
  (bind _full_wire (Variables|Default|GetFull_Wire))
  (Components|StaticMesh|SetStaticMesh _full_wire (Variables|Default|GetFullWireMesh))
  (Transformation|SetRelativeScale3D _full_wire "0.100000,0.100000,0.150000")
  (Rendering|Material|SetMaterial (Variables|Default|GetFull_Wire) 0 (Variables|Default|GetMaterail)))