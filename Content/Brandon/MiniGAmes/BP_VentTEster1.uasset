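; Vent unscrewing minigame prototype: using the vent switches to its camera, hides and locks the player, and enables mouse clicks.
; Clicking any of four screws plays a timeline that spins and slides it.
; AddScrewCompleted tallies finished screws, then triggers a delayed hide of the panel to reveal wires.
; Screw destruction and constraint breaking are disconnected; CuttingWires only stores a cursor trace hit.
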(event OnBeginCursorOver(BP_Screw1)
  (params (TouchedComponent :type Primitive%20Component%20Object%20Reference)))

(event OnBeginCursorOver(BP_Screw2)
  (params (TouchedComponent :type Primitive%20Component%20Object%20Reference)))

(event OnClicked(BP_Screw4)
  (params (TouchedComponent :type Primitive%20Component%20Object%20Reference) (ButtonPressed :type Key%20Structure))
  (bind _bp_screw4 (Variables|Default|GetBP_Screw4))
  (bind _relativelocation (Variables|/Script/Engine.SceneComponent|GetRelativeLocation _bp_screw4))
  (bind _newtrack_0 (Timeline|Timeline_3 Play)
    (:Update
      (Transformation|SetRelativeLocation _bp_screw4 (Math|Vector|MakeVector (.x _relativelocation) (* _newtrack_0 5.0) (.z _relativelocation)) false false)
      (Transformation|SetRelativeRotation (Variables|Default|GetBP_Screw4) (Math|Rotator|MakeRotator 0.0 (* _newtrack_0 1e+03) 0.0) false false))))

(event OnClicked(BP_Screw3)
  (params (TouchedComponent :type Primitive%20Component%20Object%20Reference) (ButtonPressed :type Key%20Structure))
  (bind _bp_screw3 (Variables|Default|GetBP_Screw3))
  (bind _relativelocation (Variables|/Script/Engine.SceneComponent|GetRelativeLocation _bp_screw3))
  (bind _newtrack_0 (Timeline|Timeline_2 Play)
    (:Update
      (Transformation|SetRelativeLocation _bp_screw3 (Math|Vector|MakeVector (.x _relativelocation) (* _newtrack_0 5.0) (.z _relativelocation)) false false)
      (Transformation|SetRelativeRotation (Variables|Default|GetBP_Screw3) (Math|Rotator|MakeRotator 0.0 (* _newtrack_0 1e+03) 0.0) false false))))

(event OnBeginCursorOver(BP_Screw4)
  (params (TouchedComponent :type Primitive%20Component%20Object%20Reference)))

(event OnBeginCursorOver(BP_Screw3)
  (params (TouchedComponent :type Primitive%20Component%20Object%20Reference)))

(event OnEndCursorOver(BP_Screw1)
  (params (TouchedComponent :type Primitive%20Component%20Object%20Reference)))

(event OnEndCursorOver(BP_Screw2)
  (params (TouchedComponent :type Primitive%20Component%20Object%20Reference)))

(event OnEndCursorOver(BP_Screw3)
  (params (TouchedComponent :type Primitive%20Component%20Object%20Reference)))

(event OnEndCursorOver(BP_Screw4)
  (params (TouchedComponent :type Primitive%20Component%20Object%20Reference)))

(event OnClicked(BP_Screw1)
  (params (TouchedComponent :type Primitive%20Component%20Object%20Reference) (ButtonPressed :type Key%20Structure))
  (bind _bp_screw1 (Variables|Default|GetBP_Screw1))
  (bind _relativelocation (Variables|/Script/Engine.SceneComponent|GetRelativeLocation _bp_screw1))
  (bind _newtrack_0 (Timeline|Timeline_0 Play)
    (:Update
      (Transformation|SetRelativeLocation _bp_screw1 (Math|Vector|MakeVector (.x _relativelocation) (* _newtrack_0 5.0) (.z _relativelocation)) false false)
      (Transformation|SetRelativeRotation (Variables|Default|GetBP_Screw1) (Math|Rotator|MakeRotator 0.0 (* _newtrack_0 1e+03) 0.0) false false))))

(event OnClicked(BP_Screw2)
  (params (TouchedComponent :type Primitive%20Component%20Object%20Reference) (ButtonPressed :type Key%20Structure))
  (bind _bp_screw2 (Variables|Default|GetBP_Screw2))
  (bind _relativelocation (Variables|/Script/Engine.SceneComponent|GetRelativeLocation _bp_screw2))
  (bind _newtrack_0 (Timeline|Timeline_1 Play)
    (:Update
      (Transformation|SetRelativeLocation _bp_screw2 (Math|Vector|MakeVector (.x _relativelocation) (* _newtrack_0 5.0) (.z _relativelocation)) false false)
      (Transformation|SetRelativeRotation (Variables|Default|GetBP_Screw2) (Math|Rotator|MakeRotator 0.0 (* _newtrack_0 1e+03) 0.0) false false))))

(event Custom|Make%20vent%20panel%20fall
  ;[0 1 0] Reveal the Wires by waiting 2 seconds then disables physics, collision and makes the panel invisible
  (Utilities|FlowControl|DoOnce false
    (:Completed
      (Utilities|FlowControl|Delay 2.0)
      (Physics|SetSimulatePhysics (Variables|Default|GetCube) false)
      (Collision|SetCollisionEnabled (Variables|Default|GetCube) "NoCollision")
      (Rendering|SetVisibility (Variables|Default|GetCube) false false)
      (Variables|Default|SetHasPanelCameOff true))))

(event Custom|CuttingWires
  (bind _hitactor (CallFunction|LineTraceforInteractables))
  (Variables|Default|SetHit%20Actor _hitactor))

(event Custom|Check%20Vent%20screws
  ;[0 1 0] Destroys screws and breaks their constraints
  ;;[0.15 0.15 0.15 0.5] Gets the amount of scews
  (bind _hit_actor (Variables|Default|GetHit%20Actor)
    (:then
      (bind _screwnum (Class|BPINOCASTTEST|GetScrewNum(Message) _hit_actor))
      (if (.Value (Utilities|Map|Find (Variables|Default|GetScrewMap) _screwnum))
        (switch int _screwnum
          (:1
            ;;[0.15 0.15 0.15 0.5] Screw 1
            (Utilities|FlowControl|DoOnce false))
          (:2
            ;;[0.15 0.15 0.15 0.5] Screw 2
            (Utilities|FlowControl|DoOnce false))
          (:3
            ;;[0.15 0.15 0.15 0.5] Screw 3
            (Utilities|FlowControl|DoOnce false))
          (:4
            ;;[0.15 0.15 0.15 0.5] Screw 4
            (Utilities|FlowControl|DoOnce false)))))
    (:else)))

(event EventBeginPlay
  ;[0 1 0] Seeting each screw to a specific number on begin play
)

(event EventTick
  (params (DeltaSeconds :type Float%20%28single-precision%29))
  ;[0 1 0] Event Tick - Checking if player is interacting with screws
  (if (Variables|Default|GetIsActive)
    (Variables|/Script/Engine.PlayerController|SetbShowMouseCursor (Game|GetPlayerController 0) true)))

(event EventItemUsed
  (bind _returnvalue (Game|GetPlayerController 0))
  (bind _returnvalue_2 (Game|GetPlayerCharacter 0))
  ;[0 1 0] When Vent is interacted with it changes the view of the camera to this actors camera view
  (Variables|Default|SetIsActive true)
  (Game|Player|SetViewTargetwithBlend (Game|GetPlayerController 0) self 0.0 "VTBlend_Linear" 0.0 false)
  ;[0 1 0] Making players mesh invisible, disabling player movement, setting mouse cursor to show and disbales players collision so mouse traces dont get interupted
  (Rendering|SetVisibility (Variables|/Script/Engine.Character|GetMesh _returnvalue_2) false true)
  (Input|SetIgnoreMoveInput _returnvalue true)
  (Variables|/Script/Engine.PlayerController|SetbShowMouseCursor _returnvalue true)
  (Collision|SetCollisionEnabled (Variables|/Script/Engine.Character|GetCapsuleComponent _returnvalue_2) "NoCollision")
  (Variables|/Script/Engine.PlayerController|SetbEnableClickEvents (Game|GetPlayerController 0) true))

(fn ConstructionScript)

(fn AddScrewCompleted
  (params (ScrewNumber :type Integer) (ScrewREf :type BP%20Screw%20Object%20Reference))
  ;[0 1 0] Adds the completed screw to an array and then loops through that array and checks if all are finished and if true it calls the make vent panel fall function
  (Utilities|Map|Add (Variables|Default|GetScrewMap) ScrewNumber true)
  (bind _valuepin (Utilities|Map|ForEachLoop(Map) (Variables|Default|GetScrewMap) :!label _label)
    (:then
      (if _valuepin
        (bind _result (Math|Integer|IncrementInt (LocalVariables|GetScrewIt))
          (:%20%20
            (if (>= _result (Variables|Default|GetNumberOfScrewsOnVent))
              (CallFunction|MakeVentPanelFall)
              (goto _label BreakPin))))))))

(fn LineTraceforInteractables
  (bind _returnvalue (Game|GetPlayerController 0))
  (bind (_locationx _locationy) (Game|Player|GetMousePosition _returnvalue))
  (bind (_worldlocation _worlddirection) (Class|PlayerController|DeprojectScreenPositiontoWorld _returnvalue _locationx _locationy))
  (bind _outhit (Collision|LineTraceByChannel (Transformation|GetWorldLocation (Variables|Default|GetCamera)) (+ _worldlocation (* _worlddirection 5e+02)) "TraceTypeQuery1" false 0 "ForDuration"))
  (return (.HitActor (Collision|BreakHitResult _outhit))))

(fn SetConstraintComponents
  (params (Physics%20Constraint%20Ref :type Physics%20Constraint%20Component%20Object%20Reference) (Screw%20Ref :type Primitive%20Component%20Object%20Reference))
  (Class|PhysicsConstraintComponent|SetConstrainedComponents Physics%20Constraint%20Ref Screw%20Ref "None" (Variables|Default|GetCube) "None"))

(fn SettingScrewVariables
  (params (Physics%20Constraint%20Ref :type Physics%20Constraint%20Component%20Object%20Reference) (ScrewRef :type Mesh%20Component%20Object%20Reference)))

(fn GetScrewNum
  (return 0))