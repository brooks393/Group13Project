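; BP_Screw is a minigame screw that backs a BP_Vent interaction, reporting to the vent once fully turned.
; Interact starts or pauses a timeline that slides and spins the cube mesh, resuming from where it stopped.
; On finish it calls AddScrewCompleted on the vent with its number and reference.
; A Tick mouse-trace control path also exists, but the code that enables its camera flag is disconnected.
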(event Custom|Rotate%20Screw
  (bind _cube (Variables|Default|GetCube))
  ;[0 1 0] Working
  (bind _newtrack_0 (Timeline|Timeline Play)
    (:Update
      (Transformation|SetRelativeLocation _cube (Math|Vector|MakeVector 0.0 (* _newtrack_0 1.5e+02) 0.0) false false)
      (Transformation|SetRelativeRotation _cube (Math|Rotator|MakeRotator 9e+01 (* _newtrack_0 1.45e+03) 0.0) false false))
    (:Finished
      (bind _asbp_vent (Utilities|Casting|CastToBP_Vent (Variables|Default|GetInteract_0))
        (:then
          (Default|AddScrewCompleted _asbp_vent (Variables|Default|GetScrewNumber) self))
        (:CastFailed
          (Development|PrintString "Failed"))))))

(event Custom|Destory
  (Actor|DestroyActor))

(event Custom|Pause%20Screw
  (bind _cube (Variables|Default|GetCube))
  ;[0 1 0] Working
  (bind _newtrack_0 (Timeline|Timeline Stop)
    (:Update
      (Transformation|SetRelativeLocation _cube (Math|Vector|MakeVector 0.0 (* _newtrack_0 1.5e+02) 0.0) false false)
      (Transformation|SetRelativeRotation _cube (Math|Rotator|MakeRotator 9e+01 (* _newtrack_0 1.45e+03) 0.0) false false))
    (:Finished
      (bind _asbp_vent (Utilities|Casting|CastToBP_Vent (Variables|Default|GetInteract_0))
        (:then
          (Default|AddScrewCompleted _asbp_vent (Variables|Default|GetScrewNumber) self))
        (:CastFailed
          (Development|PrintString "Failed"))))))

(event EventBeginPlay
  (Variables|Default|Setset%20original%20loc "0, 0, 0"))

(event Collision|EventActorBeginOverlap
  (params (OtherActor :type Actor%20Object%20Reference)))

(event EventINteract
  (params (Interact :type Character%20Object%20Reference) (IsStarting :type Boolean) (vent :type BP%20Vent%20Object%20Reference))
  (Variables|Default|SetInteract_0 vent)
  (if IsStarting
    (CallFunction|RotateScrew)
    (else
      (CallFunction|PauseScrew))))

(event EventTick
  (params (DeltaSeconds :type Float%20%28single-precision%29))
  (bind _returnvalue (Game|GetPlayerController 0))
  (bind (_locationx _locationy) (Game|Player|GetMousePosition _returnvalue))
  (bind (_worldlocation _worlddirection) (Class|PlayerController|DeprojectScreenPositiontoWorld _returnvalue _locationx _locationy))
  (if (Variables|Default|Getis%20camera%20active)
    (bind _outhit (Collision|LineTraceByChannel (Transformation|GetWorldLocation (Variables|Default|GetCamera)) (+ _worldlocation (* _worlddirection 5e+02)) "TraceTypeQuery3" false 0 "ForDuration" false "(R=0.000000,G=0.288002,B=1.000000,A=1.000000)" "(R=0.000000,G=1.000000,B=0.000000,A=1.000000)" 1e+01))
    (if (== (.HitActor (Collision|BreakHitResult _outhit)) self)
      (Development|PrintString "True")
      (CallFunction|RotateScrew)
      (else
        (Development|PrintString "False")
        (CallFunction|PauseScrew)))))

(fn ConstructionScript)