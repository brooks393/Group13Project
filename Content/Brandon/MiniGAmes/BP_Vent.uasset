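; Vent minigame actor where the player unscrews four screws to remove the panel and reveal wires.
; Using it switches to the vent's camera, hides the player, blocks movement and shows the cursor.
; Each tick, a cursor trace starts or stops screwing through BPI_Interact, and screws marked done in ScrewMap lose their constraints and are destroyed.
; AddScrewCompleted fills that map and, once enough screws finish, hides the panel after a delay.
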(event Custom|Make%20vent%20panel%20fall
  ;[0 1 0] Reveal the Wires by waiting 2 seconds then disables physics, collision and makes the panel invisible
  (Utilities|FlowControl|DoOnce false
    (:Completed
      (Utilities|FlowControl|Delay 2.0)
      (Physics|SetSimulatePhysics (Variables|Default|GetCube) false)
      (Collision|SetCollisionEnabled (Variables|Default|GetCube) "NoCollision")
      (Rendering|SetVisibility (Variables|Default|GetCube) false false))))

(event Custom|Check%20Vent%20screws
  ;[0 1 0] Destroys screws and breaks their constraints
  ;;[0.15 0.15 0.15 0.5] Gets the amount of scews
  (bind _hit_actor (Variables|Default|GetHit%20Actor)
    (:then
      (bind _screwnum (Class|BPINOCASTTEST|GetScrewNum(Message) _hit_actor))
      (if (.Value (Utilities|Map|Find (Variables|Default|GetScrewMap) _screwnum))
        (switch int _screwnum
          (:1
            ;;[0.15 0.15 0.15 0.5] Screw 1
            (Utilities|FlowControl|DoOnce false
              (:Completed
                (Variables|Default|GetBP_Screw1
                  (:then
                    (Class|PhysicsConstraintComponent|BreakConstraint (Variables|Default|GetScrew1Constraint))
                    (Components|DestroyComponent (Variables|Default|GetBP_Screw1)))
                  (:else)))))
          (:2
            ;;[0.15 0.15 0.15 0.5] Screw 2
            (Utilities|FlowControl|DoOnce false
              (:Completed
                (Variables|Default|GetBP_Screw2
                  (:then
                    (Class|PhysicsConstraintComponent|BreakConstraint (Variables|Default|GetScrew2Constraint))
                    (Components|DestroyComponent (Variables|Default|GetBP_Screw2)))
                  (:else)))))
          (:3
            ;;[0.15 0.15 0.15 0.5] Screw 3
            (Utilities|FlowControl|DoOnce false
              (:Completed
                (Variables|Default|GetBP_Screw3
                  (:then
                    (Class|PhysicsConstraintComponent|BreakConstraint (Variables|Default|GetScrew3Constraint))
                    (Components|DestroyComponent (Variables|Default|GetBP_Screw3)))
                  (:else)))))
          (:4
            ;;[0.15 0.15 0.15 0.5] Screw 4
            (Utilities|FlowControl|DoOnce false
              (:Completed
                (Variables|Default|GetBP_Screw4
                  (:then
                    (Class|PhysicsConstraintComponent|BreakConstraint (Variables|Default|GetScrew4Constraint))
                    (Components|DestroyComponent (Variables|Default|GetBP_Screw4)))
                  (:else))))))))
    (:else)))

(event EventBeginPlay
  ;[0 1 0] Seeting each screw to a specific number on begin play
  (bind _asbp_screw (Utilities|Casting|CastToBP_Screw (Variables|/Script/Engine.ChildActorComponent|GetChildActor (Variables|Default|GetBP_Screw1))))
  (Variables|/Game/Brandon/MiniGAmes/BP_Screw.BP_Screw_C|SetScrewNumber _asbp_screw 1)
  (bind _asbp_screw_2 (Utilities|Casting|CastToBP_Screw (Variables|/Script/Engine.ChildActorComponent|GetChildActor (Variables|Default|GetBP_Screw2))))
  (Variables|/Game/Brandon/MiniGAmes/BP_Screw.BP_Screw_C|SetScrewNumber _asbp_screw_2 2)
  (bind _asbp_screw_3 (Utilities|Casting|CastToBP_Screw (Variables|/Script/Engine.ChildActorComponent|GetChildActor (Variables|Default|GetBP_Screw3))))
  (Variables|/Game/Brandon/MiniGAmes/BP_Screw.BP_Screw_C|SetScrewNumber _asbp_screw_3 3)
  (bind _asbp_screw_4 (Utilities|Casting|CastToBP_Screw (Variables|/Script/Engine.ChildActorComponent|GetChildActor (Variables|Default|GetBP_Screw4))))
  (Variables|/Game/Brandon/MiniGAmes/BP_Screw.BP_Screw_C|SetScrewNumber _asbp_screw_4 4))

(event EventTick
  (params (DeltaSeconds :type Float%20%28single-precision%29))
  (bind _returnvalue (Game|GetPlayerController 0))
  (bind _hitresult (Game|Player|GetHitResultUnderCursorbyChannel _returnvalue "TraceTypeQuery1" true))
  (bind _hitactor (Collision|BreakHitResult _hitresult))
  ;[0 1 0] Event Tick - Checking if player is interacting with screws
  (if (Variables|Default|GetIsActive)
    (Variables|/Script/Engine.PlayerController|SetbShowMouseCursor (Game|GetPlayerController 0) true)
    ;;[0.15 0.15 0.15 0.5] Checks vent screws to see if any need to be destroyed and break constraints
    (CallFunction|CheckVentScrews)
    (if (Utilities|DoesObjectImplementInterface _hitactor "/Game/Brandon/Interfaces/BPI_Interact.BPI_Interact_C")
      (Variables|Default|SetHit%20Actor _hitactor)
      ;[0 1 0] Interacting with screw
      (if (== (Utilities|GetClass (Variables|Default|GetHit%20Actor)) "/Game/Brandon/MiniGAmes/BP_Screw.BP_Screw_C")
        (Development|PrintString "Trueee")
        (Class|BPIInteract|INteract(Message) (Variables|Default|GetHit%20Actor) 0 true self)
        (else
          (Development|PrintString "Not Trueee")))
      (else
        (Utilities|IsValid (Variables|Default|GetHit%20Actor)
          (:Is%20Valid
            (Development|PrintString "Stop iscrewing")
            (Class|BPIInteract|INteract(Message) (Variables|Default|GetHit%20Actor) 0 false self))
          (:Is%20Not%20Valid
            (Development|PrintString "Invalid")))))))

(event EventItemUsed
  (bind _returnvalue (Game|GetPlayerController 0))
  (bind _returnvalue_2 (Game|GetPlayerCharacter 0))
  ;[0 1 0] When Vent is interacted with it changes the view of the camera to this actors camera view
  (Variables|Default|SetIsActive true)
  (Game|Player|SetViewTargetwithBlend (Game|GetPlayerController 0) self 0.0 "VTBlend_Linear" 0.0 false)
  ;[0 1 0] Making players mesh invisible, disabling player movement, setting mouse cursor to show and disbales players collision so mouse traces dont get interupted
  (Rendering|SetVisibility (Variables|/Script/Engine.Character|GetMesh _returnvalue_2) false true)
  (Input|SetIgnoreMoveInput _returnvalue true)
  (Variables|/Script/Engine.PlayerController|SetbShowMouseCursor _returnvalue true)
  (Collision|SetCollisionEnabled (Variables|/Script/Engine.Character|GetCapsuleComponent _returnvalue_2) "NoCollision"))

(fn ConstructionScript)

(fn AddScrewCompleted
  (params (ScrewNumber :type Integer) (ScrewREf :type BP%20Screw%20Object%20Reference))
  ;[0 1 0] Adds the completed screw to an array and then loops through that array and checks if all are finished and if true it calls the make vent panel fall function
  (Utilities|Map|Add (Variables|Default|GetScrewMap) ScrewNumber true)
  (bind _valuepin (Utilities|Map|ForEachLoop(Map) (Variables|Default|GetScrewMap) :!label _label)
    (:then
      (if _valuepin
        (bind _result (Math|Integer|IncrementInt (LocalVariables|GetScrewIt))
          (:%20%20
            (if (>= _result (Variables|Default|GetNumberOfScrewsOnVent))
              (CallFunction|MakeVentPanelFall)
              (goto _label BreakPin))))))))

(fn GetScrewNum
  (return 0))