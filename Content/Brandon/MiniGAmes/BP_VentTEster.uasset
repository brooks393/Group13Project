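; Vent minigame test actor: using it switches to the vent's camera, hides and freezes the player, and shows the cursor.
; Hovering a screw plays a timeline that slides and spins it out and sets its physics constraint to the panel.
; Tick traces from camera through cursor, messaging interactables via BPI_Interact; constraint-breaking logic is disconnected.
; AddScrewCompleted counts finished screws, then hides the panel after a delay.
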(event OnBeginCursorOver(BP_Screw1)
  (params (TouchedComponent :type Primitive%20Component%20Object%20Reference))
  ;[0.15 0.15 0.15 0.5] Pulling Out each screw when cursor goes over them
  (CallFunction|SettingScrewVariables (Variables|Default|GetScrew1Constraint) (Variables|Default|GetBP_Screw1)))

(event OnBeginCursorOver(BP_Screw2)
  (params (TouchedComponent :type Primitive%20Component%20Object%20Reference))
  ;[0.15 0.15 0.15 0.5] Pulling Out each screw when cursor goes over them
  (CallFunction|SettingScrewVariables (Variables|Default|GetScrew2Constraint) (Variables|Default|GetBP_Screw2)))

(event OnBeginCursorOver(BP_Screw4)
  (params (TouchedComponent :type Primitive%20Component%20Object%20Reference))
  ;[0.15 0.15 0.15 0.5] Pulling Out each screw when cursor goes over them
  (CallFunction|SettingScrewVariables (Variables|Default|GetScrew4Constraint) (Variables|Default|GetBP_Screw4)))

(event OnBeginCursorOver(BP_Screw3)
  (params (TouchedComponent :type Primitive%20Component%20Object%20Reference))
  ;[0.15 0.15 0.15 0.5] Pulling Out each screw when cursor goes over them
  (CallFunction|SettingScrewVariables (Variables|Default|GetScrew3Constraint) (Variables|Default|GetBP_Screw3)))

(event Custom|Make%20vent%20panel%20fall
  ;[0 1 0] Reveal the Wires by waiting 2 seconds then disables physics, collision and makes the panel invisible
  (Utilities|FlowControl|DoOnce false
    (:Completed
      (Utilities|FlowControl|Delay 2.0)
      (Physics|SetSimulatePhysics (Variables|Default|GetPanel) false)
      (Collision|SetCollisionEnabled (Variables|Default|GetPanel) "NoCollision")
      (Rendering|SetVisibility (Variables|Default|GetPanel) false false)
      (Variables|Default|SetHasPanelCameOff true))))

(event Custom|CuttingWires
  (bind _hitactor (CallFunction|LineTraceforInteractables))
  (Variables|Default|SetHit%20Actor _hitactor))

(event Custom|Check%20Vent%20screws
  ;[0 1 0] Destroys screws and breaks their constraints
  ;;[0.15 0.15 0.15 0.5] Gets the amount of scews
  (bind _hit_actor (Variables|Default|GetHit%20Actor)
    (:then
      (bind _screwnum (Class|BPINOCASTTEST|GetScrewNum(Message) _hit_actor))
      (if (.Value (Utilities|Map|Find (Variables|Default|GetScrewMap) _screwnum))
        (switch int _screwnum
          (:1
            ;;[0.15 0.15 0.15 0.5] Screw 1
            (Utilities|FlowControl|DoOnce false))
          (:2
            ;;[0.15 0.15 0.15 0.5] Screw 2
            (Utilities|FlowControl|DoOnce false))
          (:3
            ;;[0.15 0.15 0.15 0.5] Screw 3
            (Utilities|FlowControl|DoOnce false))
          (:4
            ;;[0.15 0.15 0.15 0.5] Screw 4
            (Utilities|FlowControl|DoOnce false)))))
    (:else)))

(event Custom|PullOutScrew
  (params (ScrewRef :type Mesh%20Component%20Object%20Reference))
  (bind _newtrack_0 (Timeline|Timeline Play)
    (:Update
      (Transformation|SetRelativeLocation ScrewRef (Math|Vector|MakeVector 0.0 (* _newtrack_0 1.5e+02) 0.0) false false)
      (Transformation|SetRelativeRotation ScrewRef (Math|Rotator|MakeRotator 0.0 (* _newtrack_0 1.45e+03) 0.0) false false))))

(event EventBeginPlay
  ;[0 1 0] Seeting each screw to a specific number on begin play
)

(event EventTick
  (params (DeltaSeconds :type Float%20%28single-precision%29))
  ;[0 1 0] Event Tick - Checking if player is interacting with screws
  (if (Variables|Default|GetIsActive)
    (Variables|/Script/Engine.PlayerController|SetbShowMouseCursor (Game|GetPlayerController 0) true)
    ;;[0.15 0.15 0.15 0.5] Checks vent screws to see if any need to be destroyed and break constraints
    (CallFunction|CheckVentScrews)
    (bind _hitactor (CallFunction|LineTraceforInteractables))
    (if (Utilities|DoesObjectImplementInterface _hitactor "/Game/Brandon/Interfaces/BPI_Interact.BPI_Interact_C")
      (bind _output_get (Variables|Default|SetHit%20Actor _hitactor))
      ;;[0 1 0] Interacting with screw
      (Class|BPIInteract|CutWire(Message) _output_get)
      (else
        (Utilities|IsValid (Variables|Default|GetHit%20Actor))))))

(event EventItemUsed
  (bind _returnvalue (Game|GetPlayerController 0))
  (bind _returnvalue_2 (Game|GetPlayerCharacter 0))
  ;[0 1 0] When Vent is interacted with it changes the view of the camera to this actors camera view
  (Variables|Default|SetIsActive true)
  (Game|Player|SetViewTargetwithBlend (Game|GetPlayerController 0) self 0.0 "VTBlend_Linear" 0.0 false)
  ;[0 1 0] Making players mesh invisible, disabling player movement, setting mouse cursor to show and disbales players collision so mouse traces dont get interupted
  (Rendering|SetVisibility (Variables|/Script/Engine.Character|GetMesh _returnvalue_2) false true)
  (Input|SetIgnoreMoveInput _returnvalue true)
  (Variables|/Script/Engine.PlayerController|SetbShowMouseCursor _returnvalue true)
  (Collision|SetCollisionEnabled (Variables|/Script/Engine.Character|GetCapsuleComponent _returnvalue_2) "NoCollision"))

(fn ConstructionScript)

(fn AddScrewCompleted
  (params (ScrewNumber :type Integer) (ScrewREf :type BP%20Screw%20Object%20Reference))
  ;[0 1 0] Adds the completed screw to an array and then loops through that array and checks if all are finished and if true it calls the make vent panel fall function
  (Utilities|Map|Add (Variables|Default|GetScrewMap) ScrewNumber true)
  (bind _valuepin (Utilities|Map|ForEachLoop(Map) (Variables|Default|GetScrewMap) :!label _label)
    (:then
      (if _valuepin
        (bind _result (Math|Integer|IncrementInt (LocalVariables|GetScrewIt))
          (:%20%20
            (if (>= _result (Variables|Default|GetNumberOfScrewsOnVent))
              (CallFunction|MakeVentPanelFall)
              (goto _label BreakPin))))))))

(fn LineTraceforInteractables
  (bind _returnvalue (Game|GetPlayerController 0))
  (bind (_locationx _locationy) (Game|Player|GetMousePosition _returnvalue))
  (bind (_worldlocation _worlddirection) (Class|PlayerController|DeprojectScreenPositiontoWorld _returnvalue _locationx _locationy))
  (bind _outhit (Collision|LineTraceByChannel (Transformation|GetWorldLocation (Variables|Default|GetCamera)) (+ _worldlocation (* _worlddirection 5e+02)) "TraceTypeQuery3" false 0 "ForDuration"))
  (return (.HitActor (Collision|BreakHitResult _outhit))))

(fn SetConstraintComponents
  (params (Physics%20Constraint%20Ref :type Physics%20Constraint%20Component%20Object%20Reference) (Screw%20Ref :type Primitive%20Component%20Object%20Reference))
  (Class|PhysicsConstraintComponent|SetConstrainedComponents Physics%20Constraint%20Ref Screw%20Ref "None" (Variables|Default|GetPanel) "None"))

(fn SettingScrewVariables
  (params (Physics%20Constraint%20Ref :type Physics%20Constraint%20Component%20Object%20Reference) (ScrewRef :type Mesh%20Component%20Object%20Reference))
  (CallFunction|PullOutScrew ScrewRef)
  (CallFunction|SetConstraintComponents Physics%20Constraint%20Ref ScrewRef))

(fn GetScrewNum
  (return 0))