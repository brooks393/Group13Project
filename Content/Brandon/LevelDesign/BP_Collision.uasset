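; BP_Collision is a trigger box that teleports the player to a linked location and switches the camera.
; When an actor of the BrandonPerson class overlaps it, the player moves to TeleportLoc's Scene position and the view quickly blends to Camera.
; A HasGoneThroughACollision flag toggles on each overlap, so only every other one teleports.
; Hit events only print debug text, and a name-based BP_InsideBookTeleport lookup is left unconnected.
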(event OnComponentBeginOverlap(Box)
  (params (OverlappedComponent :type Primitive%20Component%20Object%20Reference) (OtherActor :type Actor%20Object%20Reference) (OtherComp :type Primitive%20Component%20Object%20Reference) (OtherBodyIndex :type Integer) (bFromSweep :type Boolean) (SweepResult :type Hit%20Result%20Structure%20%28by%20ref%29))
  (bind _returnvalue (Actor|GetActorOfClass "/Game/ThirdPerson/Blueprints/BrandonPerson.BrandonPerson_C"))
  (if (== (Utilities|GetClass _returnvalue) (Utilities|GetClass OtherActor))
    (if (Variables|Default|GetHasGoneThroughACollision)
      (Variables|Default|SetHasGoneThroughACollision false)
      (Utilities|FlowControl|Delay 0.2)
      (else
        (Variables|Default|SetHasGoneThroughACollision true)
        (Transformation|SetActorLocation (Game|GetPlayerCharacter 0) (Transformation|GetWorldLocation (Variables|BP_Collision_C|GetScene (Variables|Default|GetTeleportLoc))) false true)
        (Game|Player|SetViewTargetwithBlend (Game|GetPlayerController 0) (Variables|Default|Getcamera) 0.1 "VTBlend_Linear" 0.0 false)
        (Development|PrintString "Done")))
    (else
      (Development|PrintString "Bad"))))

(event OnComponentHit(Box)
  (params (HitComponent :type Primitive%20Component%20Object%20Reference) (OtherActor :type Actor%20Object%20Reference) (OtherComp :type Primitive%20Component%20Object%20Reference) (NormalImpulse :type Vector :default "0, 0, 0") (Hit :type Hit%20Result%20Structure%20%28by%20ref%29))
  (if (== OtherActor (Game|GetPlayerCharacter 0))
    (Development|PrintString "Player")))

(event EventBeginPlay)

(event Collision|EventActorBeginOverlap
  (params (OtherActor :type Actor%20Object%20Reference)))

(event EventTick
  (params (DeltaSeconds :type Float%20%28single-precision%29)))

(fn ConstructionScript)