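; BP_CollisionTeleporter is a level trigger that teleports the player to a linked teleporter and repositions a camera.
; On box overlap it checks that the other actor's class is exactly BrandonPerson, then moves player character 0 to the Scene transform of ConnectingTeleporter.
; It also teleports CameraToMove to the CameraLocationScene transform of ConectingCamera.
; Debug strings print for both player and non-player overlaps.
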(event OnComponentBeginOverlap(Box)
  (params (OverlappedComponent :type Primitive%20Component%20Object%20Reference) (OtherActor :type Actor%20Object%20Reference) (OtherComp :type Primitive%20Component%20Object%20Reference) (OtherBodyIndex :type Integer) (bFromSweep :type Boolean) (SweepResult :type Hit%20Result%20Structure%20%28by%20ref%29))
  (bind _connecting_teleporter (Variables|Default|GetConnecting%20Teleporter))
  (bind _conecting_camera (Variables|Default|GetConecting%20Camera))
  (bind _scene (Variables|BP_CollisionTeleporter_C|GetScene _connecting_teleporter))
  (bind _cameralocationscene (Variables|/Game/Brandon/LevelDesign/BP_BoxDesign.BP_BoxDesign_C|GetCameraLocationScene _conecting_camera))
  (if (== (Utilities|GetClass OtherActor) "/Game/ThirdPerson/Blueprints/BrandonPerson.BrandonPerson_C")
    (Development|PrintString "True")
    (Transformation|Teleport (Game|GetPlayerCharacter 0) (Transformation|GetWorldLocation _scene) (Transformation|GetWorldRotation _scene))
    (Transformation|Teleport (Variables|Default|GetCamera%20To%20Move) (Transformation|GetWorldLocation _cameralocationscene) (Transformation|GetWorldRotation _cameralocationscene))
    (else
      (Development|PrintString "Not P{layer overlappiung"))))

(event EventBeginPlay)

(event Collision|EventActorBeginOverlap
  (params (OtherActor :type Actor%20Object%20Reference)))

(event EventTick
  (params (DeltaSeconds :type Float%20%28single-precision%29)))

(fn ConstructionScript)