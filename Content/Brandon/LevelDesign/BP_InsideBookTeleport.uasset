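; BP_InsideBookTeleport is a placeable destination point that puts the player at its location, apparently for book-interior levels.
; Its TeleportToHere event moves the existing player character there without sweeping.
; With no valid character, it spawns a BrandonPerson, calls Possess with no pawn connected and switches the view to CorrespondingCamera.
; An unreachable duplicate of this logic does pass the spawned pawn to Possess.
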(event Custom|TeleportToHere
  (bind _returnvalue (Game|GetPlayerCharacter 0))
  (bind _returnvalue_2 (Transformation|GetActorLocation))
  (Utilities|IsValid _returnvalue
    (:Is%20Valid
      (Transformation|SetActorLocation _returnvalue _returnvalue_2 false true))
    (:Is%20Not%20Valid
      (Game|SpawnActorfromClass "/Game/ThirdPerson/Blueprints/BrandonPerson.BrandonPerson_C" (Math|Transform|MakeTransform _returnvalue_2 "0, 0, 0" "1.000000,1.000000,1.000000") "Undefined" "MultiplyWithRoot" 0 0)
      (Pawn|Possess (Game|GetPlayerController 0))
      (Game|Player|SetViewTargetwithBlend (Game|GetPlayerController 0) (Variables|Default|GetCorresponding%20Camera) 0.0 "VTBlend_Linear" 0.0 false))))

(event EventBeginPlay)

(event Collision|EventActorBeginOverlap
  (params (OtherActor :type Actor%20Object%20Reference)))

(event EventTick
  (params (DeltaSeconds :type Float%20%28single-precision%29)))

(fn ConstructionScript)